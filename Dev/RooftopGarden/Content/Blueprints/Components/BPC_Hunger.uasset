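; Hunger component that tracks a clamped hunger level, optionally decays it at day's end, and broadcasts changes, feeding and reaching zero.
; Players feed it Food items from the active inventory slot, with restore amounts read from DT_Satiation.
; The level persists as an instanced struct, or starts full without a save.
; Startup and load broadcasts wait two ticks so listeners can bind first.
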(event `OnDayEnded_Event`
  ;[1 1 1] Decay hunger at the end of the day if enabled
  (`self.DecayHunger`))

(event `self.ReceiveBeginPlay`
  (`|ExecutionSequence`
    (:`then_0`
      ;[1 1 1] Decay hunger at the end of the day if enabled
      (if (`self.DecayHungerAtEndDay`)
        (add `TimeSubsystem.OnDayEnded` (subsystem `TimeSubsystem`) (delegate `OnDayEnded_Event`))))
    (:`then_1`
      (bind _returnvalue (`GameplayStatics.DoesSaveGameExist` "save"))
      ;[1 0.8984 0.5654] Set after two ticks so everything is instantiated and others bind to hunger changed
      (if (not _returnvalue)
        (`KismetSystemLibrary.DelayUntilNextTick`)
        (`KismetSystemLibrary.DelayUntilNextTick`)
        (bind _output_get (set `self.CurrentHungerLevel` (`self.MaxHungerLevel`)))
        (`self.OnHungerChanged` _output_get (`self.GetHungerPercentage`))))))

(event `SaveableComponentInterface.LoadComponentState`
  (params (SaveData :type "Array of InstancedStruct Structure (by ref)"))
  (bind _output (`|GetArrayItem` SaveData))
  (if (`KismetArrayLibrary.Array_IsNotEmpty` SaveData)
    (`StructUtilsFunctionLibrary.IsInstancedStructValid` _output
      (:`Valid`
        (bind _value (`StructUtilsFunctionLibrary.GetInstancedStructValue` _output)
          (:`Valid`
            (bind _output_get (set `self.CurrentHungerLevel` (`.IntValue` (break `VariantDataStruct` _value))))
            (`KismetSystemLibrary.DelayUntilNextTick`)
            (`KismetSystemLibrary.DelayUntilNextTick`)
            (`self.OnHungerChanged` _output_get (`self.GetHungerPercentage`))))))))

(fn `CanPlayerFeed`
  (params (Inventory :type "InventoryComponent Object Reference"))
  (returns (Result :type Boolean))
  (bind (_slotstruct_itemid _slotstruct_quantity _slotstruct_item _slotstruct_itemtype) (break `SlotStruct` (`InventoryComponent.GetActiveSlotInfo` Inventory)))
  (return (and (not (`self.IsHungerMaxed`)) (`|EnumEquality` _slotstruct_itemtype "Food"))))

(fn `DecayHunger`
  ;[1 1 1] Only decrease hunger if hunger level is not 0
  (if (not (== (`self.CurrentHungerLevel`) 0))
    (bind _output_get (set `self.CurrentHungerLevel` (`KismetMathLibrary.Clamp` (- (`self.CurrentHungerLevel`) (`self.HungerDecayLevel`)) 0 (`self.MaxHungerLevel`))))
    (`self.OnHungerChanged` _output_get (`self.GetHungerPercentage`))
    ;[1 1 1] If hunger level has reached zero, call the event
    (if (== (`self.CurrentHungerLevel`) 0)
      (`self.OnHungerZeroed`))))

(fn `Feed`
  (params (ItemID :type Name))
  ;[1 1 1] Increase hunger level and call event
  (bind _returnvalue (`|GetDataTableRow` "/Game/Blueprints/DataTypes/DT_Satiation.DT_Satiation" ItemID)
    (:`then`
      (bind _output_get (set `self.CurrentHungerLevel` (`KismetMathLibrary.Clamp` (+ (break `/Game/Blueprints/DataTypes/S_Satiation` _returnvalue) (`self.CurrentHungerLevel`)) 0 (`self.MaxHungerLevel`))))
      (`self.OnHungerChanged` _output_get (`self.GetHungerPercentage`))
      (`self.OnFed`))))

(fn `GetHungerPercentage`
  (returns (Percentage :type "Float (double-precision)"))
  (return (/ (`KismetMathLibrary.Conv_IntToDouble` (`self.CurrentHungerLevel`)) (`self.MaxHungerLevel`))))

(fn `IsHungerMaxed`
  (returns (bool :type Boolean))
  (return (== (`self.MaxHungerLevel`) (`self.CurrentHungerLevel`))))

(fn `PlayerTryFeed`
  (params (Inventory :type "InventoryComponent Object Reference"))
  (returns (Success :type Boolean))
  (locals (ID :type Name))
  (bind _slotstruct_itemid (break `SlotStruct` (`InventoryComponent.GetActiveSlotInfo` Inventory)))
  (if (`self.CanPlayerFeed` Inventory)
    (set `local.ID` _slotstruct_itemid)
    (bind _returnvalue (`InventoryComponent.RemoveFromActiveSlot` Inventory 1 true))
    (if _returnvalue
      (`self.Feed` (`local.ID`))
      (return true)
      (else
        (return false)))))

(fn `SaveComponentState`
  (returns (OutSaveData :type "Array of InstancedStruct Structure"))
  (bind _returnvalue (`StructUtilsFunctionLibrary.MakeInstancedStruct` (make `VariantDataStruct` false (`self.CurrentHungerLevel`))))
  (return (`|MakeArray` _returnvalue)))

(fn `UpdateMaxHunger`
  (params (NewMax :type Integer))
  (bind _output_get (set `self.MaxHungerLevel` NewMax))
  (bind _output_get_2 (set `self.CurrentHungerLevel` (`KismetMathLibrary.FTrunc` (* _output_get (`self.GetHungerPercentage`)))))
  (`self.OnHungerChanged` _output_get_2 (`self.GetHungerPercentage`)))