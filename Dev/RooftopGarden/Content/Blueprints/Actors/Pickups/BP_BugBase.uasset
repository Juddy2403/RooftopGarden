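; Base pickup actor for bugs that belong to a plant, rendered with a Niagara effect.
; Interactable feedback visibility switches the effect's custom depth stencil value, presumably for highlighting.
; Interact caches the owner's PlantBugComponent, runs the parent pickup logic, then reports the pickup to that component unless the owner is a FarmingPlot.
; LoadState destroys the actor, so loading does not restore bugs.
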(event `OnVisibleChanged`
  (params (IsVisible :type Boolean))
  (bind _niagara (`self.Niagara`))
  (if IsVisible
    (`PrimitiveComponent.SetCustomDepthStencilValue` _niagara 2)
    (else
      (`PrimitiveComponent.SetCustomDepthStencilValue` _niagara 1))))

(event `self.ReceiveBeginPlay`
  (add `/Game/Blueprints/Components/BPC_InteractableFeedback.OnChangedVisible` (`self.BPC_InteractableFeedback`) (delegate `OnVisibleChanged`)))

(event `SaveableInterface.LoadState`
  (params (SaveData :type "Array of InstancedStruct Structure (by ref)"))
  (`self.K2_DestroyActor`))

(event `self.Interact`
  (params (InteractingActor :type "Actor Object Reference") (HeldItem :type "SlotStruct Structure"))
  (bind _returnvalue (`self.GetComponentByClass` (`self.GetOwner`) "/Script/RooftopGarden.PlantBugComponent"))
  (`/Engine/EditorBlueprintResources/StandardMacros.IsValid` _returnvalue
    (:`Is Valid`
      (set `self.BugOwner` _returnvalue))
    (:`Is Not Valid`
      _))
  (`parent.Interact` InteractingActor HeldItem)
  (cast `FarmingPlot` (`self.GetOwner`)
    (:`CastFailed`
      (`PlantBugComponent.BugPickedUp` (`self.BugOwner`) self))))

(fn `UserConstructionScript`
  (`parent.UserConstructionScript`))