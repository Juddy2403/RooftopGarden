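; Actor component that gives interactable objects visual feedback: a highlight and a floating key prompt.
; It toggles custom depth stencil values on the owner's meshes and spawns a camera-facing widget component showing W_TutorialText.
; When tutorials are enabled, the text fades in after a delay on becoming visible.
; Prompt text and key icon update at runtime and on input device changes, rebuilding the widget only when content differs.
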(event `InitMeshes`
  (set `self.MeshComponents` (`Actor.K2_GetComponentsByClass` (`self.GetOwner`) "/Script/Engine.MeshComponent")))

(event `self.ReceiveBeginPlay`
  (bind (_widgettransform_location _widgettransform_rotation _widgettransform_scale) (`KismetMathLibrary.BreakTransform` (`self.WidgetTransform`)))
  (bind _widgetcomponent (`self.WidgetComponent`))
  (add `InputDeviceSubsystem.OnInputHardwareDeviceChanged` (subsystem `InputDeviceSubsystem`) (delegate `OnInputHardwareDeviceChanged_Event`))
  ;[1 1 1] Constructing the widget component
  (`self.InitMeshes`)
  (bind _returnvalue (`|AddComponentByClass` (`self.GetOwner`) "/Script/UMG.WidgetComponent" false (`KismetMathLibrary.MakeTransform` (0.0 0.0 0.0) (struct) _widgettransform_scale)))
  (`SceneComponent.K2_SetWorldLocation` _returnvalue (+ _widgettransform_location (`Actor.K2_GetActorLocation` (`self.GetOwner`))) false false)
  (`PrimitiveComponent.SetMaterial` _returnvalue 0 "/Game/Materials/M_WidgetText.M_WidgetText")
  (set `self.WidgetComponent` _returnvalue)
  (bind _returnvalue_2 (`|CreateWidget` "/Game/Blueprints/Widgets/W_TutorialText.W_TutorialText_C" null "" "False" null))
  ;[1 1 1] Setting up the construct values
  (bind _output_get (set `self.Widget` _returnvalue_2))
  (`WidgetComponent.SetWidget` (`self.WidgetComponent`) _output_get)
  (`WidgetComponent.SetDrawSize` _widgetcomponent (`self.DrawSize`))
  (`PrimitiveComponent.SetCastShadow` _widgetcomponent false)
  ;;[1 0.7634 0.3449] So the keymap gets initialized
  (`KismetSystemLibrary.DelayUntilNextTick`)
  (`KismetSystemLibrary.DelayUntilNextTick`)
  (`self.UpdateText` (`self.Press/Hold`) (`self.IActionType`) (`self.ActionToDo`))
  (set `self.IsInitialized` true)
  (`SceneComponent.SetVisibility` (`self.WidgetComponent`) false false)
  (`self.Disable`))

(event `OnInputHardwareDeviceChanged_Event`
  (params (UserId :type "PlatformUserId Structure") (DeviceId :type "InputDeviceId Structure"))
  (`KismetSystemLibrary.DelayUntilNextTick`)
  (`self.UpdateText` (`self.Press/Hold`) (`self.IActionType`) (`self.ActionToDo`)))

(event `EnableTextAfterDelay`
  (`SceneComponent.SetVisibility` (`self.WidgetComponent`) true false)
  (`/Game/Blueprints/Widgets/W_TutorialText.PlayOpacityAnim` (`self.Widget`) "Forward"))

(event `UpdateText`
  (params (`Press/Hold` :type Text) (IActionType :type "InputAction Object Reference") (ActionToDo :type Text))
  ;[1 1 1] For runtime text update
  (bind _shouldupdate (`self.AssignNewText` `Press/Hold` IActionType ActionToDo))
  (if _shouldupdate
    (bind _returnvalue (`|CreateWidget` "/Game/Blueprints/Widgets/W_TutorialText.W_TutorialText_C" null (`|FormatText` "to {ActionToDo}" ActionToDo) (`self.Press/Hold`) (`self.IconTexture`)))
    (`WidgetComponent.SetWidget` (`self.WidgetComponent`) _returnvalue)
    (set `self.Widget` _returnvalue)))

(event `SetVisible`
  (if (not (`self.IsVisible`))
    (`self.SetHighlightShader`)
    (bind _output_get (set `self.IsVisible` true))
    (`self.OnChangedVisible` _output_get)
    (bind _isenabled (message `/Game/Blueprints/Interfaces/BPI_GamemodeUtilities.IsTutorialEnabled` (`GameplayStatics.GetGameMode`)))
    (if _isenabled
      (`KismetSystemLibrary.K2_SetTimer` null "EnableTextAfterDelay" (`self.TextShowDelay`)))))

(event `Enable`
  ;[1 1 1] Enable the component
  (`self.SetComponentTickEnabled` true)
  (`self.OnEnabled`)
  (if (`self.IsAutomatic`)
    (`self.SetVisible`)))

(event `self.ReceiveTick`
  (params (DeltaSeconds :type "Float (single-precision)"))
  (`self.OnTick`)
  (if (`self.IsVisible`)
    ;[1 1 1] On tick have the text face the player
    (`UtilitiesLibrary.LookAtCamera` (`self.WidgetComponent`))))

(event `DisableActiveText`
  (if (`self.IsVisible`)
    (if (`KismetSystemLibrary.K2_IsTimerActive` null "EnableTextAfterDelay")
      (`KismetSystemLibrary.K2_ClearTimer` null "EnableTextAfterDelay")
      (else
        (`/Game/Blueprints/Widgets/W_TutorialText.PlayOpacityAnim` (`self.Widget`) "Reverse")))))

(event `SetInvisible`
  (if (`self.IsVisible`)
    (`self.SetDefaultShader`)
    (bind _output_get (set `self.IsVisible` false))
    (`self.OnChangedVisible` _output_get)
    (bind _isenabled (message `/Game/Blueprints/Interfaces/BPI_GamemodeUtilities.IsTutorialEnabled` (`GameplayStatics.GetGameMode`)))
    (if _isenabled
      (if (`KismetSystemLibrary.K2_IsTimerActive` null "EnableTextAfterDelay")
        (`KismetSystemLibrary.K2_ClearTimer` null "EnableTextAfterDelay")
        (else
          (`/Game/Blueprints/Widgets/W_TutorialText.PlayOpacityAnim` (`self.Widget`) "Reverse"))))))

(event `Disable`
  ;[1 1 1] Disable the component - no need the disable visibility since the anim does that
  (`KismetSystemLibrary.K2_ClearTimer` null "EnableTextAfterDelay")
  (`self.SetComponentTickEnabled` false)
  (`self.OnDisabled`)
  (`self.SetInvisible`))

(event `UpdateShader`
  (`self.SetDefaultShader`)
  (if (`self.IsVisible`)
    (`self.SetHighlightShader`)))

(event `AddMesh`
  (params (Mesh :type "MeshComponent Object Reference"))
  (`KismetArrayLibrary.Array_Add` (`self.MeshComponents`) Mesh)
  (`self.UpdateShader`))

(event `RemoveLastMesh`
  (bind _meshcomponents (`self.MeshComponents`))
  (`self.SetDefaultShader`)
  (`KismetArrayLibrary.Array_Remove` _meshcomponents (- (`KismetArrayLibrary.Array_Length` _meshcomponents) 0))
  (`self.UpdateShader`))

(event `SetHighlightShader`
  (for _array_element (`self.MeshComponents`)
    (`/Engine/EditorBlueprintResources/StandardMacros.IsValid` _array_element
      (:`Is Valid`
        (`PrimitiveComponent.SetCustomDepthStencilValue` _array_element (`self.HighlightStencilValue`))))))

(event `SetDefaultShader`
  (for _array_element (`self.MeshComponents`)
    (`/Engine/EditorBlueprintResources/StandardMacros.IsValid` _array_element
      (:`Is Valid`
        (`PrimitiveComponent.SetCustomDepthStencilValue` _array_element (`self.DefaultStencilValue`))))))

(fn `AssignNewText`
  (params (`Press/Hold` :type Text) (IActionType :type "InputAction Object Reference") (ActionToDo :type Text))
  (returns (ShouldUpdate :type Boolean))
  (if (`self.IsInitialized`)
    (bind _icon (message `/Game/Blueprints/Interfaces/BPI_ControllerUtilities.GetKeyIcon` (`GameplayStatics.GetPlayerController` 0) IActionType))
    (if (and (`KismetTextLibrary.EqualEqual_TextText` `Press/Hold` (`self.Press/Hold`)) (== IActionType (`self.IActionType`)) (`KismetTextLibrary.EqualEqual_TextText` ActionToDo (`self.ActionToDo`)) (== _icon (`self.IconTexture`)))
      (return false)
      (else
        (set `self.Press/Hold` `Press/Hold`)
        (set `self.IActionType` IActionType)
        (set `self.ActionToDo` ActionToDo)
        (set `self.IconTexture` _icon)
        (return true)))
    (else
      (bind _icon_2 (message `/Game/Blueprints/Interfaces/BPI_ControllerUtilities.GetKeyIcon` (`GameplayStatics.GetPlayerController` 0) IActionType))
      (set `self.IconTexture` _icon_2)
      (return true))))