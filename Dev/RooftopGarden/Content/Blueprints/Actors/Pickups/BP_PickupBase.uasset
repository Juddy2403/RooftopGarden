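; Base pickup actor that adds one of its item to the interacting actor's InventoryComponent, playing a sound on success.
; When RunConstruct is set, construction finds the DT_Items row matching its own class to derive the mesh and ItemID.
; It then fits the collision box to the mesh bounds and places the feedback widget above it.
; Interaction disables that feedback before adding the item; SaveState and LoadState are empty.
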(event `self.Interact`
  (params (InteractingActor :type "Actor Object Reference") (HeldItem :type "SlotStruct Structure"))
  (bind _returnvalue (`self.GetComponentByClass` InteractingActor "/Script/RooftopGarden.InventoryComponent"))
  ;[1 1 1] On pick up
  (`/Engine/EditorBlueprintResources/StandardMacros.IsValid` _returnvalue
    (:`Is Valid`
      (`/Game/Blueprints/Components/BPC_InteractableFeedback.Disable` (`self.BPC_InteractableFeedback`))
      (bind _returnvalue_2 (`InventoryComponent.AddToInventory` _returnvalue (`self.ItemID`) 1 null))
      (if _returnvalue_2
        (`GameplayStatics.PlaySound2D` "/Game/Audio/SoundCues/SC_TakingUp.SC_TakingUp" 1.0 1.0 0.0 null null)))))

(event `SaveableInterface.LoadState`
  (params (SaveData :type "Array of InstancedStruct Structure (by ref)")))

(fn `SaveState`
  (returns (OutSaveData :type "Array of InstancedStruct Structure"))
  (return))

(fn `UserConstructionScript`
  (bind _box (`self.Box`))
  (bind (_origin _boxextent) (`KismetSystemLibrary.GetComponentBounds` (`self.StaticMesh`)))
  (bind (_returnvalue_x _returnvalue_y _returnvalue_z) (`KismetMathLibrary.BreakVector` (`BoxComponent.GetScaledBoxExtent` (`self.Box`))))
  (`parent.UserConstructionScript`)
  (if (`self.RunConstruct`)
    (`|ExecutionSequence`
      (:`then_0`
        ;[1 1 1] Set the mesh and item ID depending on the item data table
        (bind _outrownames (`DataTableFunctionLibrary.GetDataTableRowNames` "/Game/Blueprints/DataTypes/DT_Items.DT_Items"))
        (for _array_element _outrownames
          (bind _returnvalue (`|GetDataTableRow` "/Game/Blueprints/DataTypes/DT_Items.DT_Items" _array_element)
            (:`then`
              (if (== (`.ItemClass` (break `ItemStruct` _returnvalue)) (`GameplayStatics.GetObjectClass` self))
                (`StaticMeshComponent.SetStaticMesh` (`self.StaticMesh`) (`.ItemMesh` (break `ItemStruct` _returnvalue)))
                (set `self.ItemID` _array_element)
                (break))))))
      (:`then_1`
        ;[1 1 1] Set accurate collision bounds depending on the mesh
        (`BoxComponent.SetBoxExtent` _box (* _boxextent (`self.BoundsMultiplier`)) true)
        (`SceneComponent.K2_SetWorldLocation` _box _origin false false))
      (:`then_2`
        (set `/Game/Blueprints/Components/BPC_InteractableFeedback.WidgetTransform` (`KismetMathLibrary.MakeTransform` (`KismetMathLibrary.MakeVector` 0.0 0.0 (+ _returnvalue_z 30.0)) (struct) (0.02 0.02 0.02)) (`self.BPC_InteractableFeedback`))))))