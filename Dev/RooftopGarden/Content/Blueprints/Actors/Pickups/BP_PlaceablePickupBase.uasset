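; Base Blueprint for pickup items that can be carried in an inventory and placed back into the world.
; Interacting disables the feedback component and adds one item to the interactor's inventory, enabling tick and playing a sound on success.
; While ticking, it updates a placement projection of its mesh when it is the owner's active slot actor, otherwise destroying it.
; Place delegates to the projection component, stops ticking on success and plays a sound.
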(event `self.ReceiveTick`
  (params (DeltaSeconds :type "Float (single-precision)"))
  (bind _bpc_projectionplaceable (`self.BPC_ProjectionPlaceable`))
  (bind _returnvalue (`self.GetComponentByClass` (`self.GetOwner`) "/Script/RooftopGarden.InventoryComponent"))
  (bind (_bisvalid _outactor) (`InventoryComponent.GetActiveSlotActor` _returnvalue))
  (`/Engine/EditorBlueprintResources/StandardMacros.IsValid` _returnvalue
    (:`Is Valid`
      (if (and _bisvalid (== _outactor self))
        (`/Game/Blueprints/Components/BPC_ProjectionPlaceable.UpdateProjection` _bpc_projectionplaceable (`StaticMeshComponent.StaticMesh` (`self.StaticMesh`)))
        (else
          (bind _projection (`/Game/Blueprints/Components/BPC_ProjectionPlaceable.Projection` _bpc_projectionplaceable)
            (:`then`
              (`self.K2_DestroyActor` _projection))
            (:`else`)))))))

(event `/Game/Blueprints/Interfaces/BPI_Placeable.Place`
  (params (`Placing Actor` :type "Actor Object Reference"))
  (bind _success (`/Game/Blueprints/Components/BPC_ProjectionPlaceable.PlaceItem` (`self.BPC_ProjectionPlaceable`) self `Placing Actor`))
  (`self.SetActorTickEnabled` (not _success))
  (`GameplayStatics.PlaySound2D` "/Game/Audio/SoundCues/SC_TakingDown.SC_TakingDown" 1.0 1.0 0.0 null null))

(event `self.Interact`
  (params (InteractingActor :type "Actor Object Reference") (HeldItem :type "SlotStruct Structure"))
  (bind _returnvalue (`self.GetComponentByClass` InteractingActor "/Script/RooftopGarden.InventoryComponent"))
  (`/Engine/EditorBlueprintResources/StandardMacros.IsValid` _returnvalue
    (:`Is Valid`
      (`/Game/Blueprints/Components/BPC_InteractableFeedback.Disable` (`self.BPC_InteractableFeedback`))
      (bind _returnvalue_2 (`InventoryComponent.AddToInventory` _returnvalue (`self.ItemID`) 1 null))
      (`self.SetActorTickEnabled` _returnvalue_2)
      (if _returnvalue_2
        (`GameplayStatics.PlaySound2D` "/Game/Audio/SoundCues/SC_TakingUp.SC_TakingUp" 1.0 1.0 0.0 null null)))))

(fn `UserConstructionScript`
  (`parent.UserConstructionScript`))