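; BP_Trapdoor is an interactable locked trapdoor that opens when the held item is a key, which is then consumed.
; Interact disables the box collision and calls Open, which plays unlock and delayed creak sounds while a timeline swings the lid.
; A feedback component's tick shows the prompt only while the player's active inventory slot holds a key.
; SaveState and LoadState persist the unlocked flag through instanced structs, restoring only the lid rotation.
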(event `self.Interact`
  (params (InteractingActor :type "Actor Object Reference") (HeldItem :type "SlotStruct Structure"))
  (if (== HeldItem_ItemID "key")
    (`self.Open`)
    (`PrimitiveComponent.SetCollisionEnabled` (`self.Box`) "NoCollision")
    (`InventoryComponent.RemoveFromActiveSlot` (`self.GetComponentByClass` InteractingActor "/Script/RooftopGarden.InventoryComponent") 1 true)))

(event `Open`
  (`AudioComponent.Play` (`self.SW_Unlocking`) 0.2)
  (`|ExecutionSequence`
    (:`then_0`
      (set `self.IsUnlocked` true)
      (bind (_direction _lidtrack) (`Timeline|Timeline`)
        (:`Update`
          (`SceneComponent.K2_SetRelativeRotation` (`self.Lid`) (`KismetMathLibrary.MakeRotator` 0.0 (`KismetMathLibrary.Lerp` 0.0 -90.0 _lidtrack)) false false))))
    (:`then_1`
      (`KismetSystemLibrary.Delay` 0.5)
      (`AudioComponent.Play` (`self.SW_Creaking`) 0.0))))

(event `FeedbackTextCheck`
  (bind _bpc_interactablefeedback (`self.BPC_InteractableFeedback`))
  (if (`self.HasKey` (`GameplayStatics.GetPlayerPawn` 0))
    (`/Game/Blueprints/Components/BPC_InteractableFeedback.SetVisible` _bpc_interactablefeedback)
    (else
      (`/Game/Blueprints/Components/BPC_InteractableFeedback.SetInvisible` _bpc_interactablefeedback))))

(event `self.ReceiveBeginPlay`
  (add `/Game/Blueprints/Components/BPC_InteractableFeedback.OnTick` (`self.BPC_InteractableFeedback`) (delegate `FeedbackTextCheck`)))

(event `SaveableInterface.LoadState`
  (params (SaveData :type "Array of InstancedStruct Structure (by ref)"))
  (bind _value (`StructUtilsFunctionLibrary.GetInstancedStructValue` (`|GetArrayItem` SaveData))
    (:`Valid`
      (bind _output_get (set `self.IsUnlocked` (`.BoolValue` (break `VariantDataStruct` _value))))
      (if _output_get
        (`SceneComponent.K2_SetRelativeRotation` (`self.Lid`) (`KismetMathLibrary.MakeRotator` 0.0 -90.0) false false)))))

(fn `HasKey`
  (params (Actor :type "Actor Object Reference"))
  (returns (Result :type Boolean))
  (bind _returnvalue (`self.GetComponentByClass` Actor "/Script/RooftopGarden.InventoryComponent"))
  (bind _slotstruct_itemid (break `SlotStruct` (`InventoryComponent.GetActiveSlotInfo` _returnvalue)))
  (`/Engine/EditorBlueprintResources/StandardMacros.IsValid` _returnvalue
    (:`Is Valid`
      (return (== _slotstruct_itemid "key")))))

(fn `SaveState`
  (returns (OutSaveData :type "Array of InstancedStruct Structure"))
  (bind _returnvalue (`StructUtilsFunctionLibrary.MakeInstancedStruct` (make `VariantDataStruct` (`self.IsUnlocked`))))
  (return (`|MakeArray` _returnvalue)))

(fn `UserConstructionScript`)