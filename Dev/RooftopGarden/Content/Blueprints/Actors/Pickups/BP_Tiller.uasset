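; BP_Tiller is a hand tool pickup that tills farming plots and pulls weeds.
; StartAction traces for the looked-at actor, stores it as the started plot and plays dirt VFX if it is a BP_FarmingPlot.
; ActionDone sends that plot a "tiller" interact message, then clears one weed if a weed item fits into the player's inventory.
; GetAnimationMontage supplies the tilling animation.
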(event `ToolUserInterface.StartAction`
  (bind (_hitactor _returnvalue) (`UtilitiesLibrary.GetLookAtHitActor` "ECC_GameTraceChannel2"))
  (if _returnvalue
    (bind _output_get (set `self.StartedPlot` _hitactor))
    (bind _asbp_farming_plot (cast `/Game/Blueprints/Actors/BP_FarmingPlot` _output_get))
    (`/Game/Blueprints/Actors/BP_FarmingPlot.PlayDirtVFX` _asbp_farming_plot 1.2)
    (else
      (set `self.StartedPlot` null))))

(fn `ActionDone`
  (bind _returnvalue (`self.GetComponentByClass` (`GameplayStatics.GetPlayerPawn` 0) "/Script/RooftopGarden.InventoryComponent"))
  (bind _startedplot (`self.StartedPlot`)
    (:`then`
      (message `Interactable.Interact` _startedplot null (make `SlotStruct` "tiller" 1 self "Tool"))
      (bind _returnvalue_2 (`self.GetComponentByClass` _startedplot "/Script/RooftopGarden.PlantWeedComponent"))
      ;[1 1 1] If there are weeds, weed
      (`/Engine/EditorBlueprintResources/StandardMacros.IsValid` _returnvalue_2
        (:`Is Valid`
          (if (`PlantWeedComponent.HasWeeds` _returnvalue_2)
            (`/Engine/EditorBlueprintResources/StandardMacros.IsValid` _returnvalue
              (:`Is Valid`
                (bind _returnvalue_3 (`InventoryComponent.AddIDToInventory` _returnvalue "weed" 1))
                (if _returnvalue_3
                  (`PlantWeedComponent.ClearOneWeed` _returnvalue_2))))))))
    (:`else`)))

(fn `GetAnimationMontage`
  (returns (ReturnValue :type "AnimMontage Object Reference"))
  (return "/Game/Animations/AnimMontages/AM_Tilling.AM_Tilling"))

(fn `UserConstructionScript`
  (`parent.UserConstructionScript`))