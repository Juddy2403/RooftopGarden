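; Interactable tool rack that holds one tool, letting the player place their active Tool item or pick up the held one into their inventory.
; Held tools snap socket-to-socket onto the rack, with the interaction box resized around them and a feedback component updating the prompt and mesh.
; Without a save game it spawns a starting tool from DT_Items; otherwise it saves the tool's IDs and re-links the actor in RestoreRelationships.
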(event `SpawnStartItem`
  (bind _heldtoolid (`self.HeldToolID`))
  (if (!= _heldtoolid "None")
    (bind _returnvalue (`|GetDataTableRow` "/Game/Blueprints/DataTypes/DT_Items.DT_Items" _heldtoolid)
      (:`then`
        (bind _returnvalue_2 (`|SpawnActorFromClass` (`.ItemClass` (break `ItemStruct` _returnvalue)) (`KismetMathLibrary.MakeTransform` (0.0 0.0 0.0)) "Undefined" "MultiplyWithRoot" null null))
        (bind _output_get (set `self.HeldToolObj` _returnvalue_2))
        (`self.AttachTool` _output_get)))))

(event `OnFeedbackCheck`
  (bind _bpc_interactablefeedback (`self.BPC_InteractableFeedback`))
  (bind _bpc_interactablefeedback_2 (`self.BPC_InteractableFeedback`))
  (bind _returnvalue (`self.GetComponentByClass` (`GameplayStatics.GetPlayerPawn` 0) "/Script/RooftopGarden.InventoryComponent"))
  ;[0.08854 0.08854 0.08854] Feedback text setup
  (`/Engine/EditorBlueprintResources/StandardMacros.IsValid` _returnvalue
    (:`Is Valid`
      (if (and (`InventoryComponent.HasInventorySpace` _returnvalue) (!= (`self.HeldToolID`) "None"))
        (`/Game/Blueprints/Components/BPC_InteractableFeedback.UpdateText` _bpc_interactablefeedback "Press" "/Game/Input/Actions/IA_Interact.IA_Interact" "pick up")
        (`/Game/Blueprints/Components/BPC_InteractableFeedback.SetVisible` _bpc_interactablefeedback)
        (else
          (bind (_itemstruct _returnvalue_2) (`UtilitiesLibrary.GetActiveItemInfoStruct` _returnvalue))
          (if (and (`|EnumEquality` (`.ItemType` (break `ItemStruct` _itemstruct)) "Tool") _returnvalue_2)
            (`/Game/Blueprints/Components/BPC_InteractableFeedback.UpdateText` _bpc_interactablefeedback_2 "Press" "/Game/Input/Actions/IA_Interact.IA_Interact" "place")
            (`/Game/Blueprints/Components/BPC_InteractableFeedback.SetVisible` _bpc_interactablefeedback_2)
            (else
              (`/Game/Blueprints/Components/BPC_InteractableFeedback.SetInvisible` _bpc_interactablefeedback_2))))))))

(event `self.ReceiveBeginPlay`
  (bind _bpc_interactablefeedback (`self.BPC_InteractableFeedback`))
  (add `/Game/Blueprints/Components/BPC_InteractableFeedback.OnEnabled` _bpc_interactablefeedback (delegate `OnFeedbackCheck`))
  (add `/Game/Blueprints/Components/BPC_InteractableFeedback.OnTick` _bpc_interactablefeedback (delegate `OnFeedbackCheck`))
  (bind _returnvalue (`GameplayStatics.DoesSaveGameExist` "save"))
  (if (not _returnvalue)
    (`self.SpawnStartItem`)))

(event `self.Interact`
  (params (InteractingActor :type "Actor Object Reference") (HeldItem :type "SlotStruct Structure"))
  (bind _returnvalue (`self.GetComponentByClass` InteractingActor "/Script/RooftopGarden.InventoryComponent"))
  (bind _box (`self.Box`))
  (bind (_slotstruct_itemid _slotstruct_quantity _slotstruct_item) (break `SlotStruct` (`InventoryComponent.GetActiveSlotInfo` _returnvalue)))
  ;[0.05208 0.05208 0.05208] Try to place tool
  (`/Engine/EditorBlueprintResources/StandardMacros.IsValid` _returnvalue
    (:`Is Valid`
      (if (and (> _slotstruct_quantity 0) (== (`self.HeldToolID`) "None"))
        (bind _itemstruct (`UtilitiesLibrary.GetActiveItemInfoStruct` _returnvalue))
        (if (`|EnumEquality` (`.ItemType` (break `ItemStruct` _itemstruct)) "Tool")
          (set `self.HeldToolID` _slotstruct_itemid)
          (set `self.HeldToolObj` _slotstruct_item)
          (bind _returnvalue_2 (`InventoryComponent.RemoveFromActiveSlot` _returnvalue 1 false))
          (if _returnvalue_2
            (`self.AttachTool` (`self.HeldToolObj`))
            (`GameplayStatics.PlaySound2D` "/Game/Audio/SoundCues/SC_TakingDown.SC_TakingDown" 1.0 1.0 0.0 null null)))
        (else
          ;[0.0625 0.0625 0.0625] Try to add item to inventory
          (if (and (`InventoryComponent.HasInventorySpace` _returnvalue) (!= (`self.HeldToolID`) "None"))
            (bind _returnvalue_3 (`InventoryComponent.AddToInventory` _returnvalue (`self.HeldToolID`) 1 (`self.HeldToolObj`)))
            (if _returnvalue_3
              (set `self.HeldToolID` "None")
              (`/Game/Blueprints/Components/BPC_InteractableFeedback.RemoveLastMesh` (`self.BPC_InteractableFeedback`))
              (`BoxComponent.SetBoxExtent` _box (`self.CollisionBoxExtent`) true)
              (`SceneComponent.K2_SetWorldLocation` _box (`self.CollisionBoxOrigin`) false false)
              (set `self.HeldToolObj` null)
              (`GameplayStatics.PlaySound2D` "/Game/Audio/SoundCues/SC_TakingUp.SC_TakingUp" 1.0 1.0 0.0 null null))))))))

(event `AttachTool`
  (params (ToolObj :type "Actor Object Reference"))
  (bind _box (`self.Box`))
  (bind _rootcomponent (`Actor.RootComponent` ToolObj))
  (bind (_origin _boxextent) (`KismetSystemLibrary.GetComponentBounds` _rootcomponent))
  ;[0.08854 0.08854 0.08854] Attach tool to rack
  (`self.SetOwner` ToolObj self)
  (`UtilitiesLibrary.AttachComponentsSocketToSocket` _rootcomponent (`self.StaticMesh`) "ToolRackHandle" "ToolRackSlot")
  (`self.SetActorEnableCollision` ToolObj false)
  (`BoxComponent.SetBoxExtent` _box (* _boxextent 1.5) true)
  (`SceneComponent.K2_SetWorldLocation` _box _origin false false)
  (bind _asstatic_mesh_component (cast `StaticMeshComponent` _rootcomponent))
  (`/Game/Blueprints/Components/BPC_InteractableFeedback.AddMesh` (`self.BPC_InteractableFeedback`) _asstatic_mesh_component))

(event `SaveableInterface.LoadState`
  (params (SaveData :type "Array of InstancedStruct Structure (by ref)"))
  (if (`KismetArrayLibrary.Array_IsNotEmpty` SaveData)
    (bind _value (`StructUtilsFunctionLibrary.GetInstancedStructValue` (`|GetArrayItem` SaveData))
      (:`Valid`
        (bind (_boolvalue _intvalue _floatvalue _namevalue _stringvalue _id) (break `VariantDataStruct` _value))
        (set `self.HeldToolID` _namevalue)
        (set `self.ToolID` _id)))))

(event `SaveableInterface.RestoreRelationships`
  (params (ActorMap :type "Map of Guid Structure to Actor Object Reference (by ref)"))
  (bind (_value _returnvalue) (`BlueprintMapLibrary.Map_Find` ActorMap (`self.ToolID`)))
  (if _returnvalue
    (bind _output_get (set `self.HeldToolObj` _value))
    (`self.AttachTool` _output_get)
    (else
      (set `self.HeldToolID` "None"))))

(fn `SaveState`
  (returns (OutSaveData :type "Array of InstancedStruct Structure"))
  (if (!= (`self.HeldToolID`) "None")
    (bind _heldtoolobj (`self.HeldToolObj`)
      (:`then`
        (bind _returnvalue (message `SaveableInterface.GetSaveID` _heldtoolobj))
        (bind _returnvalue_2 (`StructUtilsFunctionLibrary.MakeInstancedStruct` (make `VariantDataStruct` false 0 0.0 (`self.HeldToolID`) "" _returnvalue)))
        (return (`|MakeArray` _returnvalue_2)))
      (:`else`
        _)))
  (return))

(fn `UserConstructionScript`
  (bind _box (`self.Box`))
  (`parent.UserConstructionScript`)
  (set `self.CollisionBoxExtent` (* (`BoxComponent.GetScaledBoxExtent` _box) 1.5))
  (set `self.CollisionBoxOrigin` (`SceneComponent.K2_GetComponentLocation` _box)))