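; BP_Radio is an interactable radio actor that lets the player mute or unmute the music.
; Interact calls the HUD's toggle for the music mute state through the player controller.
; On BeginPlay it binds to the feedback component's tick, which polls the HUD's muted state and updates the prompt text to show the matching action.
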(event `OnFeedbackUpdate`
  (bind _bpc_interactablefeedback (`self.BPC_InteractableFeedback`))
  (bind _newparam (message `/Game/Blueprints/Interfaces/BPI_HudUtilities.IsMusicMuted` (`PlayerController.GetHUD` (`GameplayStatics.GetPlayerController` 0))))
  (if _newparam
    (`/Game/Blueprints/Components/BPC_InteractableFeedback.UpdateText` _bpc_interactablefeedback "Press" "/Game/Input/Actions/IA_Interact.IA_Interact" "unmute music")
    (else
      (`/Game/Blueprints/Components/BPC_InteractableFeedback.UpdateText` _bpc_interactablefeedback "Press" "/Game/Input/Actions/IA_Interact.IA_Interact" "mute music"))))

(event `self.ReceiveBeginPlay`
  (add `/Game/Blueprints/Components/BPC_InteractableFeedback.OnTick` (`self.BPC_InteractableFeedback`) (delegate `OnFeedbackUpdate`)))

(event `self.Interact`
  (params (InteractingActor :type "Actor Object Reference") (HeldItem :type "SlotStruct Structure"))
  (message `/Game/Blueprints/Interfaces/BPI_HudUtilities.ToggleMuteMusic` (`PlayerController.GetHUD` (`GameplayStatics.GetPlayerController` 0))))

(fn `UserConstructionScript`)