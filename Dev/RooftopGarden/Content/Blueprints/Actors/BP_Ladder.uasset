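; Climbable ladder actor for the first-person character, with a height set per instance.
; The construction script stacks mesh segments plus a top piece, resizes the trigger box and positions begin and end points from height and offset variables.
; Overlapping the trigger passes the ladder to the character through AddBPLadderClimb.
; AttachToTheLadder snaps the character onto the ladder facing it, stops its movement and switches it to Flying mode.
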(event `self.Ladder collider.OnComponentBeginOverlap`
  (params (OverlappedComponent :type "PrimitiveComponent Object Reference") (OtherActor :type "Actor Object Reference") (OtherComp :type "PrimitiveComponent Object Reference") (OtherBodyIndex :type Integer) (bFromSweep :type Boolean) (SweepResult :type "HitResult Structure (by ref)"))
  (bind _asbp_first_person_character (cast `/Game/Blueprints/Pawns/BP_FirstPersonCharacter` OtherActor))
  (`AddComponent|NODE_AddBP_Ladder_Climb-0` :`self` _asbp_first_person_character :`Ladder` self))

(fn `AttachToTheLadder`
  (params (PlayerCharacter :type "/Game/Blueprints/Pawns/BP_FirstPersonCharacter Object Reference"))
  (bind (_returnvalue_x _returnvalue_y) (`KismetMathLibrary.BreakVector` (`self.K2_GetActorLocation`)))
  (bind (_returnvalue_x_2 _returnvalue_y_2 _returnvalue_z) (`KismetMathLibrary.BreakVector` (`self.K2_GetActorLocation` PlayerCharacter)))
  (bind _as_bp_first_person_character (`self.As BP First Person Character`))
  (bind _charactermovement (`Character.CharacterMovement` _as_bp_first_person_character))
  (bind (_returnvalue_roll _returnvalue_pitch _returnvalue_yaw) (`KismetMathLibrary.BreakRotator` (`KismetMathLibrary.FindLookAtRotation` (`self.K2_GetActorLocation` _as_bp_first_person_character) (`self.K2_GetActorLocation`))))
  (`self.K2_SetActorLocation` PlayerCharacter (+ (`KismetMathLibrary.MakeVector` _returnvalue_x _returnvalue_y _returnvalue_z) (* (`self.GetActorForwardVector`) 20.0)) false false)
  (`self.K2_SetActorRotation` _as_bp_first_person_character (`KismetMathLibrary.MakeRotator` 0.0 0.0 _returnvalue_yaw) false)
  (`CharacterMovementComponent.SetMovementMode` _charactermovement "MOVE_Flying" 0)
  (`MovementComponent.StopMovementImmediately` _charactermovement)
  (set `CharacterMovementComponent.bOrientRotationToMovement` false _charactermovement))

(fn `UserConstructionScript`
  (locals (NewLocalVar :type "Transform Structure"))
  ;[1 1 1] Ladder stacking
  (for _index (range (+ (`self.LadderHeight`) 1))
    (`AddComponent|NODE_AddStaticMeshComponent-0` :`RelativeTransform` (`KismetMathLibrary.MakeTransform` (`KismetMathLibrary.MakeVector` 0.0 0.0 (* _index (`self.HeightPerMesh`))))))
  ;[1 1 1] Add the top piece at the end of the ladder
  (`AddComponent|NODE_AddStaticMeshComponent-1` :`RelativeTransform` (`KismetMathLibrary.MakeTransform` (`KismetMathLibrary.MakeVector` 0.0 0.0 (* (+ (`self.LadderHeight`) 1) (`self.HeightPerMesh`)))))
  ;[1 1 1] Resize collider to include the whole ladder
  (`SceneComponent.K2_SetRelativeLocation` (`self.Ladder collider`) (`KismetMathLibrary.MakeVector` 30.0 0.0 (`KismetMathLibrary.Conv_IntToDouble` (* (`self.LadderHeight`) 40))) false false)
  (`BoxComponent.SetBoxExtent` (`self.Ladder collider`) (`KismetMathLibrary.MakeVector` 86.0 64.0 (`KismetMathLibrary.Conv_IntToDouble` (* (+ (`self.LadderHeight`) 4) (`self.HeightPerMesh`)))) true)
  (`SceneComponent.K2_SetRelativeLocation` (`self.Beginpoint`) (+ (`KismetMathLibrary.MakeVector` 70.0 0.0 (`KismetMathLibrary.Conv_IntToDouble` (* (`self.GroundCollHeight`) 15))) (`self.BeginPointOffset`)) false false)
  (`SceneComponent.K2_SetRelativeLocation` (`self.EndPoint`) (+ (`KismetMathLibrary.MakeVector` -30.0 0.0 (`KismetMathLibrary.Conv_IntToDouble` (* (`self.TopCollHeight`) 15))) (`self.EndPointOffset`)) false false))