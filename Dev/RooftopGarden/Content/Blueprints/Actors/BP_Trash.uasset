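; Trash bin actor that lets players throw away items from their inventory and retrieve them again.
; Interact removes one non-tool item from the active slot, records its ID and has the PhysicsItem component spawn its mesh within box limits.
; Secondary interaction returns the most recently thrown item to the inventory, using the ID array as a stack.
; When the day ends, both the stored IDs and physics items are cleared.
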(event `self.Interact`
  (params (InteractingActor :type "Actor Object Reference") (HeldItem :type "SlotStruct Structure"))
  (bind _returnvalue (`self.GetComponentByClass` InteractingActor "/Script/RooftopGarden.InventoryComponent"))
  (bind (_slotstruct_itemid _slotstruct_quantity) (break `SlotStruct` (`InventoryComponent.GetActiveSlotInfo` _returnvalue)))
  (`/Engine/EditorBlueprintResources/StandardMacros.IsValid` _returnvalue
    (:`Is Valid`
      (if (> _slotstruct_quantity 0)
        (bind (_itemstruct _returnvalue_2) (`UtilitiesLibrary.GetActiveItemInfoStruct` _returnvalue))
        (if (and _returnvalue_2 (`|EnumInequality` (`.ItemType` (break `ItemStruct` _itemstruct)) "Tool"))
          (`KismetArrayLibrary.Array_Add` (`self.ItemIDsArray`) _slotstruct_itemid)
          (`InventoryComponent.RemoveFromActiveSlot` _returnvalue 1 true)
          (`PhysicsItemComponent.SpawnActorIfWithinLimit` (`self.PhysicsItem`) (`.ItemMesh` (break `ItemStruct` _itemstruct)))
          (`GameplayStatics.PlaySound2D` "/Game/Audio/SoundCues/SC_TakingDown.SC_TakingDown" 1.0 1.0 0.0 null null))))))

(event `self.Interact_Secondary`
  (params (InteractingActor :type "Actor Object Reference (by ref)"))
  (bind _returnvalue (`self.GetComponentByClass` InteractingActor "/Script/RooftopGarden.InventoryComponent"))
  (bind _itemidsarray (`self.ItemIDsArray`))
  (bind _returnvalue_2 (`KismetArrayLibrary.Array_LastIndex` _itemidsarray))
  ;[1 1 1] On secondary action, pick up last thrown item
  (if (`KismetArrayLibrary.Array_IsNotEmpty` (`self.ItemIDsArray`))
    (`/Engine/EditorBlueprintResources/StandardMacros.IsValid` _returnvalue
      (:`Is Valid`
        (bind _returnvalue_3 (`InventoryComponent.AddIDToInventory` _returnvalue (`|GetArrayItem` _itemidsarray _returnvalue_2) 1))
        (if _returnvalue_3
          (`PhysicsItemComponent.DiscardLastItem` (`self.PhysicsItem`))
          (`KismetArrayLibrary.Array_Remove` _itemidsarray _returnvalue_2)
          (`GameplayStatics.PlaySound2D` "/Game/Audio/SoundCues/SC_TakingUp.SC_TakingUp" 1.0 1.0 0.0 null null))))))

(event `self.ReceiveBeginPlay`
  (add `TimeSubsystem.OnDayEnded` (subsystem `TimeSubsystem`) (delegate `OnDayEnded`)))

(event `OnDayEnded`
  (`PhysicsItemComponent.Reset` (`self.PhysicsItem`))
  (`KismetArrayLibrary.Array_Clear` (`self.ItemIDsArray`)))

(fn `UserConstructionScript`
  (bind _physicsitem (`self.PhysicsItem`))
  (set `PhysicsItemComponent.SpawnAreaBox` (`self.SpawnArea`) _physicsitem)
  (set `PhysicsItemComponent.SpawnLimitBox` (`self.SpawnLimit`) _physicsitem))