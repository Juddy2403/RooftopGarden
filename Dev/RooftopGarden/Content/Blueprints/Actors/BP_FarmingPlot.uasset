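; Farming plot actor that the player ploughs, plants, waters, treats and harvests, showing the plot's state visually.
; Binds to its plough, watering, bug, health and day-end events to drive soil and plant material parameters and toggle evil VFX for bugs.
; The interaction prompt derives from the player's active inventory slot, showing press or hold per action, while failed interactions send error messages to the HUD.
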(event `OnPloughed`
  (`MeshComponent.SetScalarParameterValueOnMaterials` (`self.PlotMesh`) "HasBeenPloughed" 1.0))

(event `OnWatered_Event`
  ;[1 1 1] Setting the soil color darker
  (`MeshComponent.SetScalarParameterValueOnMaterials` (`self.PlotMesh`) "HasBeenWatered" 1.0))

(event `OnPloughReset`
  (`MeshComponent.SetScalarParameterValueOnMaterials` (`self.PlotMesh`) "HasBeenPloughed" 0.0))

(event `OnSick_Event`
  (`MeshComponent.SetScalarParameterValueOnMaterials` (`self.PlantMesh`) "IsSick" 1.0))

(event `self.ReceiveBeginPlay`
  (bind _bpc_interactablefeedback (`self.BPC_InteractableFeedback`))
  (bind _plantbugcomponent (`self.PlantBugComponent`))
  (bind _plotploughcomponent (`self.PlotPloughComponent`))
  (add `PlantBugComponent.OnBugsSpawned` _plantbugcomponent (delegate `OnBugsSpawned_Event`))
  (add `PlantBugComponent.OnBugsCleared` _plantbugcomponent (delegate `OnBugsCleared_Event`))
  (add `PlantWateringComponent.OnWatered` (`self.PlantWateringComponent`) (delegate `OnWatered_Event`))
  (add `TimeSubsystem.OnDayEnded` (subsystem `TimeSubsystem`) (delegate `OnDayEnded_Event`))
  (add `/Game/Blueprints/Components/BPC_InteractableFeedback.OnEnabled` _bpc_interactablefeedback (`|CreateDelegate` :!event `InteractableFeedbackCheck`))
  (add `/Game/Blueprints/Components/BPC_InteractableFeedback.OnTick` _bpc_interactablefeedback (`|CreateDelegate` :!event `InteractableFeedbackCheck`))
  (add `PlotPloughComponent.OnPloughed` _plotploughcomponent (delegate `OnPloughed`))
  (add `PlotPloughComponent.OnPloughReset` _plotploughcomponent (delegate `OnPloughReset`))
  (add `self.OnInteractionFailed` (delegate `OnInteractionFailed_Event`))
  (add `PlantHealthComponent.OnSick` (`self.PlantHealthComponent`) (delegate `OnSick_Event`))
  (`KismetSystemLibrary.DelayUntilNextTick`)
  (`KismetSystemLibrary.DelayUntilNextTick`)
  (if (== (`PlantHealthComponent.CurrentHealth` (`self.PlantHealthComponent`)) 1)
    (`MeshComponent.SetScalarParameterValueOnMaterials` (`self.PlantMesh`) "IsSick" 1.0)))

(event `OnBugsSpawned_Event`
  (`ActorComponent.Activate` (`self.EvilVFX`) false))

(event `OnInteractionFailed_Event` :!signature `self.OnInteractionFailed`
  (params (FailText :type Text))
  (message `/Game/Blueprints/Interfaces/BPI_HudUtilities.NotifyError` (`PlayerController.GetHUD` (`GameplayStatics.GetPlayerController` 0)) FailText))

(event `OnDayEnded_Event`
  ;[1 1 1] Resetting the soil color
  (`MeshComponent.SetScalarParameterValueOnMaterials` (`self.PlotMesh`) "HasBeenWatered" 0.0))

(event `OnBugsCleared_Event`
  (`ActorComponent.Deactivate` (`self.EvilVFX`)))

(event `InteractableFeedbackCheck`
  (bind _interaction (`self.GetCurrentInteractionType`))
  (bind _bpc_interactablefeedback (`self.BPC_InteractableFeedback`))
  (bind (_press_hold _iactiontype _whattodo) (`self.GetPlotInteractionFeedbackText` _interaction))
  (if (`|EnumEquality` _interaction "none")
    (`/Game/Blueprints/Components/BPC_InteractableFeedback.SetInvisible` _bpc_interactablefeedback)
    (else
      (`/Game/Blueprints/Components/BPC_InteractableFeedback.UpdateText` _bpc_interactablefeedback _press_hold _iactiontype _whattodo)
      (`/Game/Blueprints/Components/BPC_InteractableFeedback.SetVisible` (`self.BPC_InteractableFeedback`)))))

(event `PlayDirtVFX`
  (params (Delay :type "Float (double-precision)" :default 1.0))
  (bind _dirtvfx (`self.DirtVFX`))
  (`KismetSystemLibrary.Delay` Delay)
  (`ActorComponent.Activate` _dirtvfx false)
  (`KismetSystemLibrary.Delay` 1.0)
  (`ActorComponent.Deactivate` _dirtvfx))

(fn `GetCurrentInteractionType`
  (returns (Interaction :type "EPlotInteractions Enum"))
  (bind _returnvalue (`self.GetCurrentInteraction` (`InventoryComponent.GetActiveSlotInfo` (`self.GetComponentByClass` (`GameplayStatics.GetPlayerPawn` 0) "/Script/RooftopGarden.InventoryComponent"))))
  (return _returnvalue))

(fn `GetPlotInteractionFeedbackText`
  (params (PlotInteraction :type "EPlotInteractions Enum" :default "plantSeed"))
  (returns (`Press/Hold` :type Text) (IActionType :type "InputAction Object Reference") (WhatToDo :type Text))
  (locals (`Press/HoldVar` :type Text) (IActionTypeVar :type "InputAction Object Reference") (WhatToDoVar :type Text))
  (switch `EPlotInteractions` PlotInteraction
    (:`plantSeed`
      (set `local.Press/HoldVar` "Press" :!label _label)
      (set `local.IActionTypeVar` "/Game/Input/Actions/IA_Interact.IA_Interact"))
    (:`water`
      (set `local.Press/HoldVar` "Hold" :!label _label_2)
      (set `local.IActionTypeVar` "/Game/Input/Actions/IA_Action.IA_Action"))
    (:`harvest`
      (goto _label))
    (:`plough`
      (goto _label_2))
    (:`weed`
      (goto _label_2))
    (:`useHerbicide`
      (goto _label_2))
    (:`usePesticide`
      (goto _label_2))
    (:`useFertilizer`
      (goto _label_2))
    (:`clearDeadPlant`
      (goto _label_2)))
  (bind _returnvalue (`UtilitiesLibrary.ToSentenceCase` (`|GetEnumeratorNameAsString` PlotInteraction)))
  (bind _output_get (set `local.WhatToDoVar` (`KismetTextLibrary.TextToLower` _returnvalue)))
  (return (`local.Press/HoldVar`) (`local.IActionTypeVar`) _output_get))

(fn `UserConstructionScript`)