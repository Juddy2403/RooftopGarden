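; BP_FarmingPot is a portable variant of a farming plot that can be picked up while empty and placed elsewhere.
; It extends parent interactions with pickup into the inventory, matching feedback text, and a box trace that blocks seed planting in obstructed spots.
; Pickup enables Tick, which shows a placement projection while the pot is the active slot item; successful placement disables Tick again.
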(event `self.ReceiveTick`
  (params (DeltaSeconds :type "Float (single-precision)"))
  (bind _returnvalue (`self.GetComponentByClass` (`self.GetOwner`) "/Script/RooftopGarden.InventoryComponent"))
  (bind (_bisvalid _outactor) (`InventoryComponent.GetActiveSlotActor` _returnvalue))
  ;[1 1 1] When picked up, handle projection
  (`/Engine/EditorBlueprintResources/StandardMacros.IsValid` _returnvalue
    (:`Is Valid`
      (if (and _bisvalid (== _outactor self))
        (`/Game/Blueprints/Components/BPC_ProjectionPlaceable.UpdateProjection` (`self.BPC_ProjectionPlaceable`) (`StaticMeshComponent.StaticMesh` (`self.PlotMesh`)))
        (else
          (bind _projection (`/Game/Blueprints/Components/BPC_ProjectionPlaceable.Projection` (`self.BPC_ProjectionPlaceable`))
            (:`then`
              (`self.K2_DestroyActor` _projection))
            (:`else`)))))))

(event `self.Interact`
  (params (InteractingActor :type "Actor Object Reference") (HeldItem :type "SlotStruct Structure"))
  (bind _returnvalue (`self.GetComponentByClass` InteractingActor "/Script/RooftopGarden.InventoryComponent"))
  (bind _returnvalue_2 (`self.GetCurrentInteraction` HeldItem))
  (if (`|EnumEquality` _returnvalue_2 "none")
    (if (`self.CantPlant`)
      (set `self.CantPlant` true)
      (message `/Game/Blueprints/Interfaces/BPI_HudUtilities.NotifyError` (`PlayerController.GetHUD` (`GameplayStatics.GetPlayerController` 0)) "Plant won't grow here")
      (else
        ;[1 1 1] If the plot has no plant, it can be picked up
        (if (not (`self.bHasPlant`))
          (`/Engine/EditorBlueprintResources/StandardMacros.IsValid` _returnvalue
            (:`Is Valid`
              (bind _returnvalue_3 (`InventoryComponent.AddToInventory` _returnvalue "farming_pot" 1 null))
              (if _returnvalue_3
                (`self.SetActorTickEnabled` true)
                (`GameplayStatics.PlaySound2D` "/Game/Audio/SoundCues/SC_TakingUp.SC_TakingUp" 1.0 1.0 0.0 null null)))))))
    (else
      (`parent.Interact` InteractingActor HeldItem))))

(event `/Game/Blueprints/Interfaces/BPI_Placeable.Place`
  (params (`Placing Actor` :type "Actor Object Reference"))
  ;[1 1 1] Place the item; If successful, the tick is no longer needed
  (bind _success (`/Game/Blueprints/Components/BPC_ProjectionPlaceable.PlaceItem` (`self.BPC_ProjectionPlaceable`) self `Placing Actor`))
  (`self.SetActorTickEnabled` (not _success))
  (`GameplayStatics.PlaySound2D` "/Game/Audio/SoundCues/SC_TakingDown.SC_TakingDown" 1.0 1.0 0.0 null null))

(event `InteractableFeedbackCheck2`
  (bind _bpc_interactablefeedback (`self.BPC_InteractableFeedback`))
  ;[1 1 1] Feedback text
  (if (`|EnumEquality` (`self.GetCurrentInteractionType`) "none")
    (if (`self.bHasPlant`)
      (`/Game/Blueprints/Components/BPC_InteractableFeedback.SetInvisible` _bpc_interactablefeedback)
      (else
        (`/Game/Blueprints/Components/BPC_InteractableFeedback.UpdateText` _bpc_interactablefeedback "Press" "/Game/Input/Actions/IA_Interact.IA_Interact" "pick up")
        (`/Game/Blueprints/Components/BPC_InteractableFeedback.SetVisible` _bpc_interactablefeedback)))
    (else
      (`self.InteractableFeedbackCheck`))))

(event `self.ReceiveBeginPlay`
  (bind _bpc_interactablefeedback (`self.BPC_InteractableFeedback`))
  (`parent.ReceiveBeginPlay`)
  (clear `/Game/Blueprints/Components/BPC_InteractableFeedback.OnEnabled` _bpc_interactablefeedback)
  (clear `/Game/Blueprints/Components/BPC_InteractableFeedback.OnTick` _bpc_interactablefeedback)
  (add `/Game/Blueprints/Components/BPC_InteractableFeedback.OnEnabled` _bpc_interactablefeedback (`|CreateDelegate` :!event `InteractableFeedbackCheck2`))
  (add `/Game/Blueprints/Components/BPC_InteractableFeedback.OnTick` _bpc_interactablefeedback (`|CreateDelegate` :!event `InteractableFeedbackCheck2`)))

(fn `GetCurrentInteraction`
  (params (HeldItem :type "SlotStruct Structure"))
  (returns (ReturnValue :type "EPlotInteractions Enum"))
  (bind (_origin _boxextent) (`KismetSystemLibrary.GetComponentBounds` (`self.PlantCheck`)))
  (bind _returnvalue (`parent.GetCurrentInteraction` HeldItem))
  (if (`|EnumEquality` _returnvalue "plantSeed")
    (bind (_outhit _returnvalue_2) (`KismetSystemLibrary.BoxTraceSingle` _origin _origin _boxextent (struct) "TraceTypeQuery2"))
    (if _returnvalue_2
      (set `self.CantPlant` true)
      (return "none")
      (else
        (return "plantSeed")))
    (else
      (return _returnvalue))))

(fn `UserConstructionScript`
  (`parent.UserConstructionScript`))