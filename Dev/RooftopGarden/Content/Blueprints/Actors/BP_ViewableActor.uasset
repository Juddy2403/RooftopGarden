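; BP_ViewableActor is an interactable mesh that the first-person character can toggle a camera view of.
; Interact calls the character's SwitchCameraView with a short blend and flips IsViewing.
; The interactable feedback component's tick event hides the feedback and HUD message while viewing, restoring both otherwise.
; The construction script applies the configured mesh, material and optional transform, and fits a thin box to the mesh bounds.
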(event `self.ReceiveBeginPlay`
  (add `/Game/Blueprints/Components/BPC_InteractableFeedback.OnTick` (`self.BPC_InteractableFeedback`) (delegate `OnTick_Event`)))

(event `OnTick_Event`
  (bind _bpc_interactablefeedback (`self.BPC_InteractableFeedback`))
  (bind _returnvalue (`PlayerController.GetHUD` (`GameplayStatics.GetPlayerController` 0)))
  (if (`self.IsViewing`)
    (`/Game/Blueprints/Components/BPC_InteractableFeedback.SetInvisible` _bpc_interactablefeedback)
    (message `/Game/Blueprints/Interfaces/BPI_HudUtilities.SetHUDEnabled` _returnvalue false)
    (else
      (`/Game/Blueprints/Components/BPC_InteractableFeedback.SetVisible` _bpc_interactablefeedback)
      (message `/Game/Blueprints/Interfaces/BPI_HudUtilities.SetHUDEnabled` _returnvalue true))))

(event `self.Interact`
  (params (InteractingActor :type "Actor Object Reference") (HeldItem :type "SlotStruct Structure"))
  (bind _asbp_first_person_character (cast `/Game/Blueprints/Pawns/BP_FirstPersonCharacter` InteractingActor))
  (`/Game/Blueprints/Pawns/BP_FirstPersonCharacter.SwitchCameraView` _asbp_first_person_character self 0.3)
  (`/Engine/EditorBlueprintResources/StandardMacros.FlipFlop`
    (:`A`
      (set `self.IsViewing` true))
    (:`B`
      (set `self.IsViewing` false))))

(fn `UserConstructionScript`
  (bind _staticmesh (`self.StaticMesh`))
  (bind _box (`self.Box`))
  (bind _meshworldtransform (`self.MeshWorldTransform`))
  (bind (_origin _boxextent) (`KismetSystemLibrary.GetComponentBounds` _staticmesh))
  (bind (_returnvalue_x _returnvalue_y _returnvalue_z) (`KismetMathLibrary.BreakVector` (* _boxextent 1.4)))
  (`StaticMeshComponent.SetStaticMesh` _staticmesh (`self.Mesh`))
  (`SceneComponent.K2_SetWorldLocation` _box _origin false false)
  (`BoxComponent.SetBoxExtent` _box (`KismetMathLibrary.MakeVector` _returnvalue_x 10.0 _returnvalue_z) true)
  (`PrimitiveComponent.SetMaterial` (`self.StaticMesh`) 0 (`self.MeshMaterial`))
  (if (not (== _meshworldtransform (`KismetMathLibrary.MakeTransform` (0.0 0.0 0.0))))
    (`SceneComponent.K2_SetWorldTransform` (`self.StaticMesh`) _meshworldtransform false false)))