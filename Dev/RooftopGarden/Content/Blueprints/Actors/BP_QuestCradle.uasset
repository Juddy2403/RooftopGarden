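; Quest crate where the player deposits requested items for data-table-driven quests and receives rewards.
; Interacting places needed held items as physics meshes and refreshes the note widget, or otherwise switches the camera to view the note.
; Completion closes the lid; at day end rewards spawn and the next quest loads, with the hatch toggling on player overlap.
; Saves store quest index and given items, which loading replays into the box.
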(event `InteractableFeedbackCheck`
  (bind _bpc_interactablefeedback (`self.BPC_InteractableFeedback`))
  (bind _slotstruct_itemid (break `SlotStruct` (`InventoryComponent.GetActiveSlotInfo` (`self.GetComponentByClass` (`GameplayStatics.GetPlayerPawn` 0) "/Script/RooftopGarden.InventoryComponent"))))
  (if (`self.IsCurrQuestComplete`)
    (`/Game/Blueprints/Components/BPC_InteractableFeedback.UpdateText` _bpc_interactablefeedback "Press" "/Game/Input/Actions/IA_Interact.IA_Interact" "view note" :!label _label)
    (elif (`.ReturnValue` (`BlueprintMapLibrary.Map_Find` (`self.RemainingItems`) _slotstruct_itemid))
      (`/Game/Blueprints/Components/BPC_InteractableFeedback.UpdateText` _bpc_interactablefeedback "Press" "/Game/Input/Actions/IA_Interact.IA_Interact" "place item")
      (else
        (goto _label)))))

(event `UpdateQuestItems`
  (bind _questidx (`self.QuestIDX`))
  ;[0.158 0.158 0.158] Update quest items
  (bind _outrownames (`DataTableFunctionLibrary.GetDataTableRowNames` "/Game/Blueprints/DataTypes/DT_Quest.DT_Quest"))
  (if (< _questidx (`KismetArrayLibrary.Array_Length` _outrownames))
    (bind _returnvalue (`|GetDataTableRow` "/Game/Blueprints/DataTypes/DT_Quest.DT_Quest" (`|GetArrayItem` _outrownames _questidx))
      (:`then`
        (bind _output_get (set `self.QuestItems` _returnvalue))
        (`PhysicsItemComponent.Reset` (`self.PhysicsItem`))
        (bind _output_get_2 (set `self.RemainingItems` (`.RequestedItemIDS_4_CC673BE440E74376EAE0ABB92E3901B6` (break `/Game/Blueprints/DataTypes/S_Quest` _output_get))))
        (bind _returnvalue_2 (`|CreateWidget` "/Game/Blueprints/Widgets/W_QuestNote.W_QuestNote_C" null _output_get_2))
        (`WidgetComponent.SetWidget` (`self.W_Note`) _returnvalue_2)))
    (else
      (clear `TimeSubsystem.OnDayEnded` (subsystem `TimeSubsystem`))
      (set `self.IsCurrQuestComplete` true)
      (`PhysicsItemComponent.Reset` (`self.PhysicsItem`)))))

(event `self.ReceiveBeginPlay`
  (bind _bpc_interactablefeedback (`self.BPC_InteractableFeedback`))
  (add `TimeSubsystem.OnDayEnded` (subsystem `TimeSubsystem`) (delegate `OnDayEnded_Event`))
  (add `/Game/Blueprints/Components/BPC_InteractableFeedback.OnEnabled` _bpc_interactablefeedback (`|CreateDelegate` :!event `InteractableFeedbackCheck`))
  (add `/Game/Blueprints/Components/BPC_InteractableFeedback.OnTick` _bpc_interactablefeedback (`|CreateDelegate` :!event `InteractableFeedbackCheck`))
  (`KismetSystemLibrary.DelayUntilNextTick`)
  (`self.UpdateQuestItems`))

(event `OnDayEnded_Event`
  ;[0.1719 0.1719 0.1719] On day ended event
  (if (`self.IsCurrQuestComplete`)
    (set `self.IsCurrQuestComplete` false)
    (`self.SpawnReward`)
    (`/Engine/EditorBlueprintResources/StandardMacros.IncrementInt` (`self.QuestIDX`)
      (:`  `
        (`self.UpdateQuestItems`)
        (set `self.ShouldOpenHatch` true)))))

(event `self.Interact`
  (params (InteractingActor :type "Actor Object Reference") (HeldItem :type "SlotStruct Structure"))
  (bind _itemid (break `SlotStruct` HeldItem))
  (bind _returnvalue (`self.GetComponentByClass` InteractingActor "/Script/RooftopGarden.InventoryComponent"))
  (if (`self.IsCurrQuestComplete`)
    (bind _asbp_first_person_character (cast `/Game/Blueprints/Pawns/BP_FirstPersonCharacter` InteractingActor))
    (`/Game/Blueprints/Pawns/BP_FirstPersonCharacter.SwitchCameraView` _asbp_first_person_character self 0.3)
    (elif (`.ReturnValue` (`BlueprintMapLibrary.Map_Find` (`self.RemainingItems`) _itemid))
      (bind _itemstruct (`UtilitiesLibrary.GetActiveItemInfoStruct` _returnvalue))
      (`self.PlaceItemInBox` _returnvalue (`.ItemMesh` (break `ItemStruct` _itemstruct)) _itemid)
      (if (`self.CheckQuest`)
        (set `self.IsCurrQuestComplete` true)
        (`self.CloseHatch`))
      (else
        (bind _asbp_first_person_character_2 (cast `/Game/Blueprints/Pawns/BP_FirstPersonCharacter` InteractingActor))
        (`/Game/Blueprints/Pawns/BP_FirstPersonCharacter.SwitchCameraView` _asbp_first_person_character_2 self 0.3)))))

(event `PlaceItemInBox`
  (params (InventoryComp :type "InventoryComponent Object Reference") (StaticMesh :type "StaticMesh Object Reference") (ItemID :type Name))
  (bind _remainingitems (`self.RemainingItems`))
  (bind _returnvalue (- (`BlueprintMapLibrary.Map_Find` _remainingitems ItemID) 1))
  (`/Engine/EditorBlueprintResources/StandardMacros.IsValid` InventoryComp
    (:`Is Valid`
      (`InventoryComponent.RemoveFromActiveSlot` InventoryComp 1 true))
    (:`Is Not Valid`
      _))
  (`PhysicsItemComponent.SpawnActorIfWithinLimit` (`self.PhysicsItem`) StaticMesh)
  (if (> _returnvalue 0)
    (`BlueprintMapLibrary.Map_Add` _remainingitems ItemID _returnvalue)
    (else
      (`BlueprintMapLibrary.Map_Remove` _remainingitems ItemID)))
  (bind _returnvalue_2 (`|CreateWidget` "/Game/Blueprints/Widgets/W_QuestNote.W_QuestNote_C" null (`self.RemainingItems`)))
  (`WidgetComponent.SetWidget` (`self.W_Note`) _returnvalue_2))

(event `SpawnReward`
  (bind (_questitems_requesteditemids _questitems_rewardeditemids) (break `/Game/Blueprints/DataTypes/S_Quest` (`self.QuestItems`)))
  (bind _rewardspawnbox (`self.RewardSpawnBox`))
  (bind _keys (`BlueprintMapLibrary.Map_Keys` _questitems_rewardeditemids))
  (for _array_element _keys
    (for _ (range 1 (+ (`BlueprintMapLibrary.Map_Find` _questitems_rewardeditemids _array_element) 1))
      (bind _returnvalue (`|GetDataTableRow` "/Game/Blueprints/DataTypes/DT_Items.DT_Items" _array_element)
        (:`then`
          (`|SpawnActorFromClass` (`.ItemClass` (break `ItemStruct` _returnvalue)) (`KismetMathLibrary.MakeTransform` (`KismetMathLibrary.RandomPointInBoundingBox` (`SceneComponent.K2_GetComponentLocation` _rewardspawnbox) (/ (`BoxComponent.GetScaledBoxExtent` _rewardspawnbox) 2.0))) "Undefined" "MultiplyWithRoot" null null))))))

(event `CloseHatch`
  ;[1 1 1] Hatch animation
  (`AudioComponent.Play` (`self.SW_Creaking`) 0.0)
  (bind _isa (`/Engine/EditorBlueprintResources/StandardMacros.FlipFlop`)
    (:`A`
      (bind (_direction _lidtrack) (`Timeline|Lid_Timeline` :!label _label_2)
        (:`Update`
          (`SceneComponent.K2_SetRelativeRotation` (`self.Lid`) (`KismetMathLibrary.MakeRotator` 180.0 (`KismetMathLibrary.Lerp` (`self.LidStartRotation`) (`self.LidEndRotation`) _lidtrack) 180.0) false false))
        (:`Finished`
          (if _isa
            (`AudioComponent.Play` (`self.SW_Close`) 0.0)))))
    (:`B`
      (goto _label_2 :!via `Reverse`))))

(event `self.PlayerCollider.OnComponentBeginOverlap`
  (params (OverlappedComponent :type "PrimitiveComponent Object Reference") (OtherActor :type "Actor Object Reference") (OtherComp :type "PrimitiveComponent Object Reference") (OtherBodyIndex :type Integer) (bFromSweep :type Boolean) (SweepResult :type "HitResult Structure (by ref)"))
  (if (and (== OtherActor (`GameplayStatics.GetPlayerPawn` 0)) (`self.ShouldOpenHatch`))
    (`self.CloseHatch`)
    (set `self.ShouldOpenHatch` false)))

(event `SaveableInterface.LoadState`
  (params (SaveData :type "Array of InstancedStruct Structure (by ref)"))
  (bind _output (`|GetArrayItem` SaveData))
  (if (`KismetArrayLibrary.Array_IsNotEmpty` SaveData)
    (`StructUtilsFunctionLibrary.IsInstancedStructValid` _output
      (:`Valid`
        (bind _value (`StructUtilsFunctionLibrary.GetInstancedStructValue` _output)
          (:`Valid`
            (bind (_questidx _givenitems) (break `QuestSaveDataStruct` _value))
            (set `self.QuestIDX` _questidx)
            (`KismetSystemLibrary.DelayUntilNextTick`)
            (`KismetSystemLibrary.DelayUntilNextTick`)
            (bind _keys (`BlueprintMapLibrary.Map_Keys` _givenitems))
            (for _array_element _keys
              (bind _returnvalue (`|GetDataTableRow` "/Game/Blueprints/DataTypes/DT_Items.DT_Items" _array_element)
                (:`then`
                  (for _ (range 1 (+ (`BlueprintMapLibrary.Map_Find` _givenitems _array_element) 1))
                    (`self.PlaceItemInBox` null (`.ItemMesh` (break `ItemStruct` _returnvalue)) _array_element)))))))))))

(fn `CheckQuest`
  (returns (IsComplete :type Boolean))
  (if (`BlueprintMapLibrary.Map_IsEmpty` (`self.RemainingItems`))
    (return true)
    (else
      (return false))))

(fn `SaveState`
  (returns (OutSaveData :type "Array of InstancedStruct Structure"))
  (locals (GivenItems :type "Map of Name to Object Object Reference"))
  (bind _questitems_requesteditemids (break `/Game/Blueprints/DataTypes/S_Quest` (`self.QuestItems`)))
  (bind _remainingitems (`self.RemainingItems`))
  (bind _givenitems (`local.GivenItems`))
  (bind _keys (`BlueprintMapLibrary.Map_Keys` _questitems_requesteditemids))
  (for _array_element _keys
    (if (`BlueprintMapLibrary.Map_Contains` _remainingitems _array_element)
      (bind _value (`BlueprintMapLibrary.Map_Find` _questitems_requesteditemids _array_element))
      (`BlueprintMapLibrary.Map_Add` _givenitems _array_element (- _value (`BlueprintMapLibrary.Map_Find` _remainingitems _array_element)))
      (else
        (`BlueprintMapLibrary.Map_Add` _givenitems _array_element _value))))
  (bind _returnvalue (`StructUtilsFunctionLibrary.MakeInstancedStruct` (make `QuestSaveDataStruct` (`self.QuestIDX`) (`local.GivenItems`))))
  (return (`|MakeArray` _returnvalue)))

(fn `UserConstructionScript`
  (bind _physicsitem (`self.PhysicsItem`))
  (bind (_returnvalue_roll _returnvalue_pitch) (`KismetMathLibrary.BreakRotator` (`SceneComponent.K2_GetComponentRotation` (`self.Lid`))))
  (set `PhysicsItemComponent.SpawnAreaBox` (`self.SpawnArea`) _physicsitem)
  (set `PhysicsItemComponent.SpawnLimitBox` (`self.SpawnLimit`) _physicsitem)
  (set `self.LidStartRotation` _returnvalue_pitch)
  (`PrimitiveComponent.SetCastShadow` (`self.W_Note`) false))