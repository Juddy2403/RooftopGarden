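; Actor component that shows a floating item name and quantity label on its owner, likely a basket.
; BeginPlay builds a world widget component with W_BasketText, then hides and disables it.
; UpdateText recreates the widget only when values change, while Enable and Disable toggle tick and drive opacity-animated visibility, with auto-show optional.
; While visible, Tick offsets and rotates the label toward whichever of four world-axis sides faces the player.
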(event `self.ReceiveBeginPlay`
  (bind (_widgettransform_location _widgettransform_rotation _widgettransform_scale) (`KismetMathLibrary.BreakTransform` (`self.WidgetTransform`)))
  (bind _widgetcomponent (`self.WidgetComponent`))
  ;[1 1 1] Constructing the widget component
  (bind _returnvalue (`|AddComponentByClass` (`self.GetOwner`) "/Script/UMG.WidgetComponent" false (`KismetMathLibrary.MakeTransform` (0.0 0.0 0.0) (struct) _widgettransform_scale)))
  (bind _output_get (set `self.OriginLocation` (+ _widgettransform_location (`Actor.K2_GetActorLocation` (`self.GetOwner`)))))
  (`SceneComponent.K2_SetWorldLocation` _returnvalue _output_get false false)
  (`PrimitiveComponent.SetMaterial` _returnvalue 0 "/Game/Materials/M_WidgetText.M_WidgetText")
  (set `self.WidgetComponent` _returnvalue)
  (bind _returnvalue_2 (`|CreateWidget` "/Game/Blueprints/Widgets/W_BasketText.W_BasketText_C" null "None" "None"))
  ;[1 1 1] Setting up the construct values
  (bind _output_get_2 (set `self.Widget` _returnvalue_2))
  (`WidgetComponent.SetWidget` (`self.WidgetComponent`) _output_get_2)
  (`WidgetComponent.SetDrawSize` _widgetcomponent (`self.DrawSize`))
  (`PrimitiveComponent.SetCastShadow` _widgetcomponent false)
  ;;[1 0.7634 0.3449] So the keymap gets initialized
  (`KismetSystemLibrary.DelayUntilNextTick`)
  (`KismetSystemLibrary.DelayUntilNextTick`)
  (`self.UpdateText` "None")
  (`SceneComponent.SetVisibility` (`self.WidgetComponent`) false false)
  (`self.Disable`))

(event `UpdateText`
  (params (ItemName :type Name) (Quantity :type Integer))
  ;[1 1 1] For runtime text update
  (if (`self.ShouldEdit` ItemName Quantity)
    (set `self.ItemName` ItemName)
    (set `self.Quantity` Quantity)
    (bind _returnvalue (`|CreateWidget` "/Game/Blueprints/Widgets/W_BasketText.W_BasketText_C" null (`KismetTextLibrary.Conv_NameToText` ItemName) (`KismetTextLibrary.Conv_IntToText` Quantity)))
    (`WidgetComponent.SetWidget` (`self.WidgetComponent`) _returnvalue)
    (set `self.Widget` _returnvalue)))

(event `SetVisible`
  (if (not (`self.IsVisible`))
    (`SceneComponent.SetVisibility` (`self.WidgetComponent`) true false)
    (`/Game/Blueprints/Widgets/W_BasketText.PlayOpacityAnim` (`self.Widget`) "Forward")
    (bind _output_get (set `self.IsVisible` true))
    (`self.OnChangedVisible` _output_get)))

(event `Enable`
  ;[1 1 1] Enable the component
  (`self.SetComponentTickEnabled` true)
  (`self.OnEnabled`)
  (if (`self.IsAutomatic`)
    (`self.SetVisible`)))

(event `self.ReceiveTick`
  (params (DeltaSeconds :type "Float (single-precision)"))
  (bind _widgettransform_location (`KismetMathLibrary.BreakTransform` (`self.WidgetTransform`)))
  (bind _widgetcomponent (`self.WidgetComponent`))
  (`self.OnTick`)
  (if (`self.IsVisible`)
    (bind (_output _rotation) (`self.GetPlayerOffset` 30.0))
    (`SceneComponent.K2_SetWorldLocation` _widgetcomponent (+ (`Actor.K2_GetActorLocation` (`self.GetOwner`)) _output _widgettransform_location) false false)
    (`SceneComponent.K2_SetWorldRotation` _widgetcomponent _rotation false false)))

(event `SetInvisible`
  (if (`self.IsVisible`)
    (`/Game/Blueprints/Widgets/W_BasketText.PlayOpacityAnim` (`self.Widget`) "Reverse")
    (bind _output_get (set `self.IsVisible` false))
    (`self.OnChangedVisible` _output_get)))

(event `Disable`
  ;[1 1 1] Disable the component - no need the disable visibility since the anim does that
  (`self.SetComponentTickEnabled` false)
  (`self.OnDisabled`)
  (`self.SetInvisible`))

(fn `GetPlayerOffset`
  (params (OffsetLen :type "Float (double-precision)"))
  (returns (Output :type "Vector Structure") (Rotation :type "Rotator Structure"))
  (bind _returnvalue (* OffsetLen -1.0))
  (bind (_returnvalue_x _returnvalue_y) (`KismetMathLibrary.BreakVector` (`KismetMathLibrary.Normal` (- (`Actor.K2_GetActorLocation` (`GameplayStatics.GetPlayerPawn` 0)) (`Actor.K2_GetActorLocation` (`self.GetOwner`))))))
  (if (> (`KismetMathLibrary.Abs` _returnvalue_x) (`KismetMathLibrary.Abs` _returnvalue_y))
    (if (> _returnvalue_x 0.0)
      (return (`KismetMathLibrary.MakeVector` OffsetLen))
      (else
        (return (`KismetMathLibrary.MakeVector` _returnvalue) (struct :`Yaw` 180.0))))
    (elif (> _returnvalue_y 0.0)
      (return (`KismetMathLibrary.MakeVector` 0.0 OffsetLen) (struct :`Yaw` 90.0))
      (else
        (return (`KismetMathLibrary.MakeVector` 0.0 _returnvalue) (struct :`Yaw` -90.0))))))

(fn `ShouldEdit`
  (params (Name :type Name) (Quantity :type Integer))
  (returns (Result :type Boolean))
  (return (not (and (== Name (`self.ItemName`)) (== Quantity (`self.Quantity`))))))