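; BP_Fertilizer is a usable pickup item that fertilizes the plot the player looks at, using a spray bottle animation.
; StartAction traces for the looked-at plot, and ActionDone calls UseFertilizer on its PlantGrowthComponent.
; A successful use consumes a charge from the consumable resource component, while a refusal shows an already-fertilized HUD error.
; When the resource runs out, the item removes itself from the owner's active inventory slot and is destroyed.
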(event `self.StartAction`
  (bind (_hitactor _returnvalue) (`UtilitiesLibrary.GetLookAtHitActor` "ECC_GameTraceChannel2"))
  (if _returnvalue
    (set `self.Plot` _hitactor)
    (else
      (set `self.Plot` null))))

(event `self.ActionDone`
  (bind _plot (`self.Plot`)
    (:`then`
      (if (`/Game/Blueprints/Components/BPC_ConsumableResource.HasAny` (`self.BPC_ConsumableResource`))
        (bind _returnvalue (`PlantGrowthComponent.UseFertilizer` (`self.GetComponentByClass` _plot "/Script/RooftopGarden.PlantGrowthComponent")))
        (if _returnvalue
          (`/Game/Blueprints/Components/BPC_ConsumableResource.Use` (`self.BPC_ConsumableResource`))
          (else
            (message `/Game/Blueprints/Interfaces/BPI_HudUtilities.NotifyError` (`PlayerController.GetHUD` (`GameplayStatics.GetPlayerController` 0)) "Fertilized already")))))
    (:`else`)))

(event `self.ReceiveBeginPlay`
  (add `/Game/Blueprints/Components/BPC_ConsumableResource.OnRanOut` (`self.BPC_ConsumableResource`) (delegate `Kill`)))

(event `Kill`
  (`InventoryComponent.RemoveFromActiveSlot` (`self.GetComponentByClass` (`self.GetOwner`) "/Script/RooftopGarden.InventoryComponent") 1 true))

(fn `GetAnimationMontage`
  (returns (ReturnValue :type "AnimMontage Object Reference"))
  (return "/Game/Animations/AnimMontages/AM_SprayBottle.AM_SprayBottle"))

(fn `UserConstructionScript`
  (`parent.UserConstructionScript`))