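; Watering can tool that waters plants and refills at a water tank, tracking water in a consumable resource component.
; StartAction traces the looked-at actor to choose filling or watering, timing the Niagara spray or reporting an empty can; GetAnimationMontage picks the matching montage.
; ActionDone refills, or spends water to message the target and call its PlantWateringComponent.
; An exact BP_PlantBase hit instead triggers a joke cat warning and hiss.
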(event `ToolUserInterface.StartAction`
  (bind _niagara (`self.Niagara`))
  (bind _result (`/Game/Blueprints/Components/BPC_ConsumableResource.HasAny` (`self.BPC_ConsumableResource`)))
  (bind (_hitactor _returnvalue) (`UtilitiesLibrary.GetLookAtHitActor` "ECC_GameTraceChannel2"))
  (if _returnvalue
    (if (== (`GameplayStatics.GetObjectClass` _hitactor) "/Game/Blueprints/Actors/BP_WaterTank.BP_WaterTank_C")
      (set `self.IsFilling` true)
      (elif _result
        (set `self.PlantToWater` _hitactor)
        (set `self.IsFilling` false :!label _label)
        (if _result
          (`KismetSystemLibrary.Delay` 0.5)
          (`ActorComponent.Activate` _niagara false)
          (`KismetSystemLibrary.Delay` 1.0)
          (`ActorComponent.Deactivate` _niagara)
          (else
            (message `/Game/Blueprints/Interfaces/BPI_HudUtilities.NotifyError` (`PlayerController.GetHUD` (`GameplayStatics.GetPlayerController` 0)) "Out of water" :!label _label_2)
            (`KismetSystemLibrary.DelayUntilNextTick`)
            (`Character.StopAnimMontage` (`GameplayStatics.GetPlayerCharacter` 0) null)))
        (else
          (goto _label_2))))
    (else
      (set `self.PlantToWater` null)
      (goto _label))))

(fn `ActionDone`
  (bind _hitactor (`UtilitiesLibrary.GetLookAtHitActor` "ECC_GameTraceChannel2"))
  (if (== (`GameplayStatics.GetObjectClass` _hitactor) "/Game/Blueprints/Actors/BP_PlantBase.BP_PlantBase_C")
    (message `/Game/Blueprints/Interfaces/BPI_HudUtilities.NotifyError` (`PlayerController.GetHUD` (`GameplayStatics.GetPlayerController` 0)) "Please do not the cat!")
    (bind _asbp_plant_base (cast `/Game/Blueprints/Actors/BP_PlantBase` _hitactor))
    (`/Game/Blueprints/Actors/BP_PlantBase.PlaySound` _asbp_plant_base "/Game/Audio/SoundCues/SC_CatHiss.SC_CatHiss")
    (elif (`self.IsFilling`)
      (`self.SecondaryAction`)
      (else
        (bind _planttowater (`self.PlantToWater`)
          (:`then`
            (bind _success (`/Game/Blueprints/Components/BPC_ConsumableResource.Use` (`self.BPC_ConsumableResource`)))
            (if _success
              (message `Interactable.Interact` _planttowater null (make `SlotStruct` "watering_can" 1 self "Tool"))
              (bind _returnvalue (`self.GetComponentByClass` _planttowater "/Script/RooftopGarden.PlantWateringComponent"))
              (`/Engine/EditorBlueprintResources/StandardMacros.IsValid` _returnvalue
                (:`Is Valid`
                  (`PlantWateringComponent.Water` _returnvalue)))))
          (:`else`))))))

(fn `GetAnimationMontage`
  (returns (ReturnValue :type "AnimMontage Object Reference"))
  (bind (_hitactor _returnvalue) (`UtilitiesLibrary.GetLookAtHitActor` "ECC_GameTraceChannel2"))
  (if (and _returnvalue (== (`GameplayStatics.GetObjectClass` _hitactor) "/Game/Blueprints/Actors/BP_WaterTank.BP_WaterTank_C"))
    (return "/Game/Animations/AnimMontages/AM_WatercanFill.AM_WatercanFill")
    (else
      (return "/Game/Animations/AnimMontages/AM_Watering.AM_Watering"))))

(fn `SecondaryAction`
  (`/Game/Blueprints/Components/BPC_ConsumableResource.Fill` (`self.BPC_ConsumableResource`)))

(fn `UserConstructionScript`
  (`parent.UserConstructionScript`))