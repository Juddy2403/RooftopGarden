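; Placement component that previews an item as a ghost projection where the player looks and places it from the inventory.
; UpdateProjection spawns, moves or destroys a BP_ProjectionActor from a look-at trace, rejecting spots where an unrotated, mesh-bounds box trace hits.
; RotateProjection turns the preview in 90-degree steps.
; PlaceItem removes one from the active InventoryComponent slot, then moves the given actor to the preview's location and rotation.
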(event `UpdateProjection`
  (params (Mesh :type "StaticMesh Object Reference"))
  (bind (_hitresult _returnvalue) (`UtilitiesLibrary.GetLookAtOutHit` "ECC_GameTraceChannel3"))
  (if _returnvalue
    (bind _projection (`self.Projection`)
      (:`then`
        (bind _returnvalue_2 (+ (`.Location` (`GameplayStatics.BreakHitResult` _hitresult)) (0.0 0.0 2.0)))
        (if (`self.BoxCollisionCheck` _returnvalue_2 Mesh)
          (`Actor.K2_DestroyActor` (`self.Projection`))
          (else
            (`Actor.K2_SetActorLocation` _projection _returnvalue_2 false false))))
      (:`else`
        (`self.SpawnProjection` _returnvalue_2 Mesh)))
    (else
      (bind _projection_2 (`self.Projection`)
        (:`then`
          (`Actor.K2_DestroyActor` _projection_2))
        (:`else`)))))

(fn `BoxCollisionCheck`
  (params (Location :type "Vector Structure") (Mesh :type "StaticMesh Object Reference"))
  (returns (DidCollide :type Boolean))
  (bind (_returnvalue_x _returnvalue_y _returnvalue_z) (`KismetMathLibrary.BreakVector` (/ (`KismetMathLibrary.GetBoxSize` (`StaticMesh.GetBoundingBox` Mesh)) 2.0)))
  (bind _returnvalue (+ (+ Location (0.0 0.0 2.0)) (`KismetMathLibrary.MakeVector` 0.0 0.0 _returnvalue_z)))
  (bind (_outhit _returnvalue_2) (`KismetSystemLibrary.BoxTraceSingle` _returnvalue _returnvalue (`KismetMathLibrary.MakeVector` _returnvalue_x _returnvalue_y _returnvalue_z) (struct) "TraceTypeQuery2"))
  (return _returnvalue_2))

(fn `PlaceItem`
  (params (Actor :type "Actor Object Reference") (PlacingActor :type "Actor Object Reference"))
  (returns (Success :type Boolean))
  (bind _returnvalue (`Actor.GetComponentByClass` PlacingActor "/Script/RooftopGarden.InventoryComponent"))
  (bind _projection (`self.Projection`)
    (:`then`
      (`/Engine/EditorBlueprintResources/StandardMacros.IsValid` _returnvalue
        (:`Is Valid`
          (bind _returnvalue_2 (`InventoryComponent.RemoveFromActiveSlot` _returnvalue 1 false))
          (if _returnvalue_2
            (`Actor.K2_SetActorLocationAndRotation` Actor (`Actor.K2_GetActorLocation` _projection) (`Actor.K2_GetActorRotation` _projection) false false)
            (`Actor.K2_DestroyActor` (`self.Projection`))
            (return true)
            (else
              _)))
        (:`Is Not Valid`
          _))
      (return false))
    (:`else`
      (return false))))

(fn `RotateProjection`
  (bind _projection (`self.Projection`)
    (:`then`
      (`Actor.K2_AddActorWorldRotation` _projection (struct :`Yaw` 90.0) false false))
    (:`else`)))

(fn `SpawnProjection`
  (params (SpawnLocation :type "Vector Structure") (SpawnMesh :type "StaticMesh Object Reference"))
  (returns (Success :type Boolean))
  (if (`self.BoxCollisionCheck` SpawnLocation SpawnMesh)
    (return false)
    (else
      (bind _returnvalue (`|SpawnActorFromClass` "/Game/Blueprints/Actors/BP_ProjectionActor.BP_ProjectionActor_C" (`KismetMathLibrary.MakeTransform` SpawnLocation) "AlwaysSpawn" "MultiplyWithRoot" null SpawnMesh null))
      (`/Engine/EditorBlueprintResources/StandardMacros.IsValid` _returnvalue
        (:`Is Valid`
          (set `self.Projection` _returnvalue)
          (return true))
        (:`Is Not Valid`
          (return false))))))