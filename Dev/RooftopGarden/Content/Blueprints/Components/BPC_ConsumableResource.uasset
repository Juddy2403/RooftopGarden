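; Actor component that tracks a consumable integer resource which can be used in steps and refilled to its maximum.
; Use subtracts a step, clamped at zero, and reports success, while Fill restores the maximum.
; Both broadcast the new fill ratio through OnQuantityUpdated, and Use also fires OnRanOut on reaching zero.
; Quantity is saved and restored through component state hooks as a variant instanced struct.
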(event `SaveableComponentInterface.LoadComponentState`
  (params (SaveData :type "Array of InstancedStruct Structure (by ref)"))
  (bind _value (`StructUtilsFunctionLibrary.GetInstancedStructValue` (`|GetArrayItem` SaveData))
    (:`Valid`
      (set `self.Quantity` (`.IntValue` (break `VariantDataStruct` _value))))))

(fn `Fill`
  (if (!= (`self.Quantity`) (`self.MaxQuantity`))
    (set `self.Quantity` (`self.MaxQuantity`))
    (`self.OnQuantityUpdated` (`self.GetPercentage`))))

(fn `GetPercentage`
  (returns (Result :type "Float (double-precision)"))
  (return (/ (`KismetMathLibrary.Conv_IntToDouble` (`self.Quantity`)) (`self.MaxQuantity`))))

(fn `HasAny`
  (returns (Result :type Boolean))
  (return (> (`self.Quantity`) 0)))

(fn `SaveComponentState`
  (returns (OutSaveData :type "Array of InstancedStruct Structure"))
  (bind _returnvalue (`StructUtilsFunctionLibrary.MakeInstancedStruct` (make `VariantDataStruct` false (`self.Quantity`))))
  (return (`|MakeArray` _returnvalue)))

(fn `Use`
  (returns (Success :type Boolean))
  (if (`self.HasAny`)
    (set `self.Quantity` (`KismetMathLibrary.Clamp` (- (`self.Quantity`) (`self.Step`)) 0 (`self.MaxQuantity`)))
    (`self.OnQuantityUpdated` (`self.GetPercentage`))
    (if (== (`self.Quantity`) 0)
      (`self.OnRanOut`))
    (return true)
    (else
      (return false))))