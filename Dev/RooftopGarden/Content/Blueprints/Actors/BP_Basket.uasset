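; BP_Basket is an interactable basket that stores one type of non-tool item at a time.
; Interact deposits the held item or, when hand and basket are empty, adds the basket to the inventory, while secondary interact takes an item back.
; A PhysicsItem component spawns meshes within box limits and supplies the count, with tick-bound widgets showing contents and prompts.
; Item ID and count are saved, and loading respawns the meshes from DT_Items.
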(event `PlaceItemInBasket`
  (params (ItemID :type Name) (ItemName :type Name) (InventoryComp :type "InventoryComponent Object Reference") (StaticMesh :type "StaticMesh Object Reference"))
  (`self.UpdateItemID` ItemID ItemName)
  (`InventoryComponent.RemoveFromActiveSlot` InventoryComp 1 true)
  (`PhysicsItemComponent.SpawnActorIfWithinLimit` (`self.PhysicsItem`) StaticMesh)
  (`self.UpdateItemCount`)
  (`GameplayStatics.PlaySound2D` "/Game/Audio/SoundCues/SC_TakingDown.SC_TakingDown" 1.0 1.0 0.0 null null))

(event `PickUpItem`
  (params (InventoryComp :type "InventoryComponent Object Reference"))
  (bind _physicsitem (`self.PhysicsItem`))
  (bind _returnvalue (`InventoryComponent.AddIDToInventory` InventoryComp (`self.HeldItemID`) 1))
  (if _returnvalue
    (`PhysicsItemComponent.DiscardLastItem` _physicsitem)
    (`self.UpdateItemCount`)
    (if (== (`PhysicsItemComponent.TotalHeldItems` _physicsitem) 0)
      (`self.UpdateItemID` "None" "None")
      (`GameplayStatics.PlaySound2D` "/Game/Audio/SoundCues/SC_TakingUp.SC_TakingUp" 1.0 1.0 0.0 null null))))

(event `self.Interact`
  (params (InteractingActor :type "Actor Object Reference") (HeldItem :type "SlotStruct Structure"))
  (bind _itemid (break `SlotStruct` HeldItem))
  (bind _returnvalue (`self.GetComponentByClass` InteractingActor "/Script/RooftopGarden.InventoryComponent"))
  (`/Engine/EditorBlueprintResources/StandardMacros.IsValid` _returnvalue
    (:`Is Valid`
      ;[0.07812 0.07812 0.07812] If the basket is empty, and the player has a non tool item in hand, place it in basket
      (bind (_itemstruct _returnvalue_2) (`UtilitiesLibrary.GetActiveItemInfoStruct` _returnvalue))
      ;[1 0.7097 0.2625] If the inventory slot is not empty
      (if _returnvalue_2
        (if (and (`|EnumInequality` (`.ItemType` (break `ItemStruct` _itemstruct)) "Tool") (`self.Check Item ID Validity` _itemid))
          (`self.PlaceItemInBasket` _itemid (break `ItemStruct` _itemstruct) _returnvalue (`.ItemMesh` (break `ItemStruct` _itemstruct))))
        (elif (== (`self.HeldItemID`) "None")
          (bind _returnvalue_3 (`InventoryComponent.AddToInventory` _returnvalue "basket" 1 null))
          (if _returnvalue_3
            (`self.SetActorTickEnabled` true)
            (`GameplayStatics.PlaySound2D` "/Game/Audio/SoundCues/SC_TakingUp.SC_TakingUp" 1.0 1.0 0.0 null null)))))))

(event `UpdateItemCount`
  ;[1 1 1] Display item count number
  (set `self.Quantity` (`PhysicsItemComponent.TotalHeldItems` (`self.PhysicsItem`))))

(event `/Game/Blueprints/Interfaces/BPI_SecondInteract.Interact_Secondary`
  (params (InteractingActor :type "Actor Object Reference (by ref)"))
  (bind _returnvalue (`self.GetComponentByClass` InteractingActor "/Script/RooftopGarden.InventoryComponent"))
  ;[1 1 1] On secondary action, pick up item from basket
  (if (> (`PhysicsItemComponent.TotalHeldItems` (`self.PhysicsItem`)) 0)
    (`/Engine/EditorBlueprintResources/StandardMacros.IsValid` _returnvalue
      (:`Is Valid`
        (`self.PickUpItem` _returnvalue)))))

(event `UpdateItemID`
  (params (ItemID :type Name) (ItemName :type Name))
  (set `self.HeldItemID` ItemID)
  (if (== ItemName "None")
    (set `self.ItemName` "None")
    (else
      (set `self.ItemName` ItemName))))

(event `SaveableInterface.LoadState`
  (params (SaveData :type "Array of InstancedStruct Structure (by ref)"))
  (bind _output (`|GetArrayItem` SaveData))
  ;[0.1476 0.1476 0.1476 1 23] Loading data
  (if (`KismetArrayLibrary.Array_IsNotEmpty` SaveData)
    (if (`StructUtilsFunctionLibrary.IsValid_InstancedStruct` _output)
      (bind _value (`StructUtilsFunctionLibrary.GetInstancedStructValue` _output)
        (:`Valid`
          (`KismetSystemLibrary.DelayUntilNextTick`)
          (bind (_boolvalue _intvalue _floatvalue _namevalue) (break `VariantDataStruct` _value))
          (if (!= _namevalue "None")
            (bind _output_get (set `self.HeldItemID` _namevalue))
            (bind _returnvalue (`|GetDataTableRow` "/Game/Blueprints/DataTypes/DT_Items.DT_Items" _output_get)
              (:`then`
                (set `self.ItemName` (break `ItemStruct` _returnvalue))
                (for _ (range 1 (+ _intvalue 1))
                  (`PhysicsItemComponent.SpawnActorIfWithinLimit` (`self.PhysicsItem`) (`.ItemMesh` (break `ItemStruct` _returnvalue)))
                  (`self.UpdateItemCount`))))))))))

(event `OnFeedbackCheck`
  (bind _bpc_interactablefeedback (`self.BPC_InteractableFeedback`))
  (bind _bpc_interactablefeedback_2 (`self.BPC_InteractableFeedback`))
  (bind _returnvalue (`self.GetComponentByClass` (`GameplayStatics.GetPlayerPawn` 0) "/Script/RooftopGarden.InventoryComponent"))
  (bind _slotstruct_itemid (break `SlotStruct` (`InventoryComponent.GetActiveSlotInfo` _returnvalue)))
  ;[0.08854 0.08854 0.08854] Feedback text setup
  (`/Engine/EditorBlueprintResources/StandardMacros.IsValid` _returnvalue
    (:`Is Valid`
      (bind (_itemstruct _returnvalue_2) (`UtilitiesLibrary.GetActiveItemInfoStruct` _returnvalue))
      (if _returnvalue_2
        (if (and (`|EnumInequality` (`.ItemType` (break `ItemStruct` _itemstruct)) "Tool") (`self.Check Item ID Validity` _slotstruct_itemid))
          (`/Game/Blueprints/Components/BPC_InteractableFeedback.UpdateText` _bpc_interactablefeedback_2 "Press" "/Game/Input/Actions/IA_Interact.IA_Interact" "place item")
          (`/Game/Blueprints/Components/BPC_InteractableFeedback.SetVisible` _bpc_interactablefeedback_2))
        (elif (!= (`self.HeldItemID`) "None")
          (`/Game/Blueprints/Components/BPC_InteractableFeedback.UpdateText` _bpc_interactablefeedback "Press" "/Game/Input/Actions/IA_Action.IA_Action" "pick up item")
          (`/Game/Blueprints/Components/BPC_InteractableFeedback.SetVisible` _bpc_interactablefeedback)
          (else
            (`/Game/Blueprints/Components/BPC_InteractableFeedback.UpdateText` _bpc_interactablefeedback "Press" "/Game/Input/Actions/IA_Interact.IA_Interact" "pick up")))))))

(event `self.ReceiveBeginPlay`
  ;[0.08854 0.08854 0.08854] Feedback text setup
  (add `/Game/Blueprints/Components/BPC_InteractableFeedback.OnTick` (`self.BPC_InteractableFeedback`) (delegate `OnFeedbackCheck`))
  (add `/Game/Blueprints/Components/BPC_BasketText.OnTick` (`self.BPC_BasketText`) (delegate `BasketWidgetUpdate`)))

(event `BasketWidgetUpdate`
  (bind _bpc_baskettext (`self.BPC_BasketText`))
  (bind _quantity (`self.Quantity`))
  ;[0.08854 0.08854 0.08854] Feedback text setup
  (if (> _quantity 0)
    (`/Game/Blueprints/Components/BPC_BasketText.UpdateText` _bpc_baskettext (`self.ItemName`) _quantity)
    (`/Game/Blueprints/Components/BPC_BasketText.SetVisible` _bpc_baskettext)
    (else
      (`/Game/Blueprints/Components/BPC_BasketText.SetInvisible` (`self.BPC_BasketText`)))))

(fn `Check Item ID Validity`
  (params (ItemID :type Name))
  (returns (Valid :type Boolean))
  (bind _helditemid (`self.HeldItemID`))
  ;[1 1 1] If the active slot has an item and its of the same type the basket currently holds (if any)
  (return (or (== _helditemid "None") (== _helditemid ItemID))))

(fn `SaveState`
  (returns (OutSaveData :type "Array of InstancedStruct Structure"))
  (bind _returnvalue (`StructUtilsFunctionLibrary.MakeInstancedStruct` (make `VariantDataStruct` false (`PhysicsItemComponent.TotalHeldItems` (`self.PhysicsItem`)) 0.0 (`self.HeldItemID`))))
  (return (`|MakeArray` _returnvalue)))

(fn `UserConstructionScript`
  (bind _physicsitem (`self.PhysicsItem`))
  (`parent.UserConstructionScript`)
  (set `PhysicsItemComponent.SpawnAreaBox` (`self.SpawnArea`) _physicsitem)
  (set `PhysicsItemComponent.SpawnLimitBox` (`self.SpawnLimit`) _physicsitem)
  (set `/Game/Blueprints/Components/BPC_InteractableFeedback.WidgetTransform` (`KismetMathLibrary.MakeTransform` (0.0 0.0 70.0) (struct) (0.02 0.02 0.02)) (`self.BPC_InteractableFeedback`)))