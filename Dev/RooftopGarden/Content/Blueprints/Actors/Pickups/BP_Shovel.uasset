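; Shovel tool actor that digs and ploughs farming plots using a digging montage.
; StartAction traces for the looked-at actor, caches it as StartedPlot and plays dirt VFX if it is a BP_FarmingPlot.
; ActionDone sends that cached actor an interact message identifying the shovel as a Tool.
; It then ploughs the soil through the actor's PlotPloughComponent, if present and not already ploughed.
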(event `ToolUserInterface.StartAction`
  (bind (_hitactor _returnvalue) (`UtilitiesLibrary.GetLookAtHitActor` "ECC_GameTraceChannel2"))
  (if _returnvalue
    (bind _output_get (set `self.StartedPlot` _hitactor))
    (bind _asbp_farming_plot (cast `/Game/Blueprints/Actors/BP_FarmingPlot` _output_get))
    (`/Game/Blueprints/Actors/BP_FarmingPlot.PlayDirtVFX` _asbp_farming_plot 1.4)
    (else
      (set `self.StartedPlot` null))))

(fn `ActionDone`
  (bind _startedplot (`self.StartedPlot`)
    (:`then`
      (message `Interactable.Interact` _startedplot null (make `SlotStruct` "shovel" 1 self "Tool"))
      (bind _returnvalue (`self.GetComponentByClass` _startedplot "/Script/RooftopGarden.PlotPloughComponent"))
      ;[1 1 1] Plough soil if it hasnt been ploughed already
      (`/Engine/EditorBlueprintResources/StandardMacros.IsValid` _returnvalue
        (:`Is Valid`
          (if (not (`PlotPloughComponent.HasBeenPloughed` _returnvalue))
            (`PlotPloughComponent.PloughSoil` _returnvalue)))))
    (:`else`)))

(fn `GetAnimationMontage`
  (returns (ReturnValue :type "AnimMontage Object Reference"))
  (return "/Game/Animations/AnimMontages/AM_Digging.AM_Digging"))

(fn `UserConstructionScript`
  (`parent.UserConstructionScript`))