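; BP_PlantBase is the Vorp plant, a cat-voiced creature the player feeds and pets.
; A hunger component drives feeding and, once hunger hits zero, arms a death collision that plays an eating cutscene and loses the game.
; DT_VorpGrowth rows set mesh, animations and hunger decay by day.
; Each day end checks growth and scatters up to two weighted-random seeds; a looping timer plays hunger-dependent sounds.
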(event `PlaySound`
  (params (Sound :type "SoundBase Object Reference"))
  (bind _sound (`self.Sound`))
  (`AudioComponent.SetSound` _sound Sound)
  (`AudioComponent.Play` _sound 0.0)
  (`KismetSystemLibrary.K2_ClearTimer` null "PlayRandomSound")
  (`KismetSystemLibrary.K2_SetTimer` null "PlayRandomSound" (`self.SoundTimeInterval`) true))

(event `PlayRandomSound`
  (bind _sound (`self.Sound`))
  (if (<= (`/Game/Blueprints/Components/BPC_Hunger.CurrentHungerLevel` (`self.BPC_Hunger`)) 5)
    (`AudioComponent.SetSound` _sound "/Game/Audio/SoundWaves/SFX/SW_CatHiss.SW_CatHiss")
    (elif (== (`KismetMathLibrary.RandomInteger` 20) 0)
      (`AudioComponent.SetSound` _sound "/Game/Audio/SoundCues/SC_CatMeow.SC_CatMeow")
      (else
        (`AudioComponent.SetSound` _sound "/Game/Audio/SoundCues/SC_CatPurr.SC_CatPurr"))))
  (`AudioComponent.Play` _sound 0.0))

(event `self.DeathCollision.OnComponentBeginOverlap`
  (params (OverlappedComponent :type "PrimitiveComponent Object Reference") (OtherActor :type "Actor Object Reference") (OtherComp :type "PrimitiveComponent Object Reference") (OtherBodyIndex :type Integer) (bFromSweep :type Boolean) (SweepResult :type "HitResult Structure (by ref)"))
  (if (`self.PlayerDied`)
    (bind _asbp_first_person_character (cast `/Game/Blueprints/Pawns/BP_FirstPersonCharacter` (`GameplayStatics.GetPlayerPawn` 0)))
    (`/Game/Blueprints/Pawns/BP_FirstPersonCharacter.SwitchCameraView` _asbp_first_person_character self 3.0)
    (`KismetSystemLibrary.Delay` 1.0)
    (`|PlayMontage` (`self.SkeletalMesh`) (`.FeedAnim_24_A6D3E21542A8AF230539E0B9D5FA0FAE` (break `/Game/Blueprints/DataTypes/S_VorpGrowthStages` (`self.GrowthData`))) 0.4
      (:`OnCompleted`
        (message `/Game/Blueprints/Interfaces/BPI_GamemodeUtilities.Lose` (`GameplayStatics.GetGameMode`))))))

(event `OnHungerZeroed_Event`
  (set `self.PlayerDied` true))

(event `OnFed`
  (bind _sound (`self.Sound`))
  (`|PlayMontage` (`self.SkeletalMesh`) (`.FeedAnim_24_A6D3E21542A8AF230539E0B9D5FA0FAE` (break `/Game/Blueprints/DataTypes/S_VorpGrowthStages` (`self.GrowthData`)))
    (:`then`
      (`KismetSystemLibrary.Delay` 0.2)
      (`AudioComponent.SetSound` _sound "/Game/Audio/SoundCues/SC_VorpEating.SC_VorpEating")
      (`AudioComponent.Play` _sound 0.0))))

(event `self.ReceiveBeginPlay`
  (bind _bpc_interactablefeedback (`self.BPC_InteractableFeedback`))
  (bind _bpc_hunger (`self.BPC_Hunger`))
  (bind (_growthdata_nextgrowthday _growthdata_nextgrowthstage _growthdata_hungerdecay) (break `/Game/Blueprints/DataTypes/S_VorpGrowthStages` (`self.GrowthData`)))
  (`KismetSystemLibrary.K2_SetTimer` null "PlayRandomSound" (`self.SoundTimeInterval`) true)
  (add `TimeSubsystem.OnDayEnded` (subsystem `TimeSubsystem`) (delegate `OnDayEnded_Event`))
  (add `/Game/Blueprints/Components/BPC_Hunger.OnHungerZeroed` _bpc_hunger (delegate `OnHungerZeroed_Event`))
  (add `/Game/Blueprints/Components/BPC_Hunger.OnFed` _bpc_hunger (delegate `OnFed`))
  (add `/Game/Blueprints/Components/BPC_InteractableFeedback.OnEnabled` _bpc_interactablefeedback (`|CreateDelegate` :!event `InteractableFeedbackCheck`))
  (add `/Game/Blueprints/Components/BPC_InteractableFeedback.OnTick` _bpc_interactablefeedback (`|CreateDelegate` :!event `InteractableFeedbackCheck`))
  (`KismetSystemLibrary.DelayUntilNextTick`)
  (`KismetSystemLibrary.DelayUntilNextTick`)
  (set `self.Inventory` (`self.GetComponentByClass` (`GameplayStatics.GetPlayerPawn` 0) "/Script/RooftopGarden.InventoryComponent"))
  (bind _outrownames (`DataTableFunctionLibrary.GetDataTableRowNames` "/Game/Blueprints/DataTypes/DT_VorpGrowth.DT_VorpGrowth"))
  (for _array_element _outrownames
    (bind _returnvalue (`|GetDataTableRow` "/Game/Blueprints/DataTypes/DT_VorpGrowth.DT_VorpGrowth" _array_element)
      (:`then`
        (if (< (`TimeSubsystem.CurrentDay` (subsystem `TimeSubsystem`)) (`.NextGrowthDay_25_638DD21D4C3363A492CF24B090C4CD02` (break `/Game/Blueprints/DataTypes/S_VorpGrowthStages` _returnvalue)))
          (set `self.GrowthData` _returnvalue)
          (`self.UpdateGrowth`)
          (break)))))
  (if (== _growthdata_hungerdecay 0)
    (bind _returnvalue_2 (`|GetDataTableRow` "/Game/Blueprints/DataTypes/DT_VorpGrowth.DT_VorpGrowth" "3")
      (:`then`
        (set `self.GrowthData` _returnvalue_2)
        (`self.UpdateGrowth`)
        (if (== (`/Game/Blueprints/Components/BPC_Hunger.CurrentHungerLevel` (`self.BPC_Hunger`)) 0)
          (set `self.PlayerDied` true))))))

(event `OnDayEnded_Event`
  (`self.CheckGrowth`)
  ;[1 1 1] Plant creates 0 to 2 seeds at end of day
  (for _ (range (+ (`KismetMathLibrary.RandomIntegerInRange` 0 2) 1))
    (`|SpawnActorFromClass` (`self.GetRandomSeed`) (`KismetMathLibrary.MakeTransform` (`self.GetSeedPoint`)) "AdjustIfPossibleButAlwaysSpawn" "MultiplyWithRoot" null null)))

(event `self.Interact`
  (params (InteractingActor :type "Actor Object Reference") (HeldItem :type "SlotStruct Structure"))
  (if (`|EnumEquality` HeldItem_ItemType "Bug")
    (`InventoryComponent.RemoveFromActiveSlot` (`self.GetComponentByClass` InteractingActor "/Script/RooftopGarden.InventoryComponent") 1 true)
    (`self.OnFed`)
    (`KismetSystemLibrary.Delay` 1.0)
    (`self.PlaySound` "/Game/Audio/SoundCues/SC_CatHiss.SC_CatHiss")
    (`ActorComponent.Activate` (`self.Burp`) true)
    (else
      (bind _success (`/Game/Blueprints/Components/BPC_Hunger.PlayerTryFeed` (`self.BPC_Hunger`) (`self.Inventory`)))
      (if _success
        (`KismetSystemLibrary.Delay` 1.0)
        (`self.PlaySound` "/Game/Audio/SoundCues/SC_CatPurr.SC_CatPurr")))))

(event `CheckGrowth`
  (bind (_nextgrowthday _nextgrowthstage) (break `/Game/Blueprints/DataTypes/S_VorpGrowthStages` (`self.GrowthData`)))
  (if (== _nextgrowthday (`TimeSubsystem.CurrentDay` (subsystem `TimeSubsystem`)))
    (bind _returnvalue (`|GetDataTableRow` "/Game/Blueprints/DataTypes/DT_VorpGrowth.DT_VorpGrowth" _nextgrowthstage)
      (:`then`
        (set `self.GrowthData` _returnvalue)
        (`self.UpdateGrowth`)))))

(event `InteractableFeedbackCheck`
  (bind _bpc_interactablefeedback (`self.BPC_InteractableFeedback`))
  (bind _inventory (`self.Inventory`))
  (bind (_slotstruct_itemid _slotstruct_quantity _slotstruct_item _slotstruct_itemtype) (break `SlotStruct` (`InventoryComponent.GetActiveSlotInfo` _inventory)))
  (if (`InventoryComponent.GetActiveSlotActor` _inventory)
    (if (or (`|EnumEquality` _slotstruct_itemtype "Food") (`|EnumEquality` _slotstruct_itemtype "Bug"))
      (`/Game/Blueprints/Components/BPC_InteractableFeedback.UpdateText` _bpc_interactablefeedback "Press" "/Game/Input/Actions/IA_Interact.IA_Interact" "feed")
      (`/Game/Blueprints/Components/BPC_InteractableFeedback.SetVisible` _bpc_interactablefeedback)
      (else
        (`/Game/Blueprints/Components/BPC_InteractableFeedback.SetInvisible` _bpc_interactablefeedback)))
    (else
      (`/Game/Blueprints/Components/BPC_InteractableFeedback.UpdateText` _bpc_interactablefeedback "Hold" "/Game/Input/Actions/IA_Action.IA_Action" "pet")
      (`/Game/Blueprints/Components/BPC_InteractableFeedback.SetVisible` _bpc_interactablefeedback))))

(event `UpdateGrowth`
  (bind _skeletalmesh (`self.SkeletalMesh`))
  (bind (_nextgrowthday _nextgrowthstage _hungerdecay _mesh _animbp) (break `/Game/Blueprints/DataTypes/S_VorpGrowthStages` (`self.GrowthData`)))
  (`SkeletalMeshComponent.SetSkeletalMeshAsset` _skeletalmesh _mesh)
  (`SkeletalMeshComponent.SetAnimInstanceClass` _skeletalmesh _animbp)
  (set `/Game/Blueprints/Components/BPC_Hunger.HungerDecayLevel` _hungerdecay (`self.BPC_Hunger`)))

(event `/Game/Blueprints/Interfaces/BPI_SecondInteract.Interact_Secondary`
  (params (InteractingActor :type "Actor Object Reference (by ref)"))
  (bind _ascharacter (cast `Character` InteractingActor))
  (bind _notifyname (`|PlayMontage` (`Character.Mesh` _ascharacter) "/Game/Animations/AnimMontages/AM_Petting.AM_Petting" 2.0)
    (:`OnNotifyBegin`
      (if (== _notifyname "Pet")
        (`|PlayMontage` (`self.SkeletalMesh`) (`.PetAnim_23_D8E0E99B4E74B6D169838B8C1F3A2D20` (break `/Game/Blueprints/DataTypes/S_VorpGrowthStages` (`self.GrowthData`))))))))

(fn `GetRandomSeed`
  (returns (Seed :type "Actor Class Reference"))
  (locals (Sum :type Integer) (Min :type Integer) (RandomValue :type Integer) (Max :type Integer))
  (bind _seedspawnchancemap (`self.SeedSpawnChanceMap`))
  (bind _randomvalue (`local.RandomValue`))
  (bind _values (`BlueprintMapLibrary.Map_Values` (`self.SeedSpawnChanceMap`)))
  (for _array_element _values
    (set `local.Sum` (+ _array_element (`local.Sum`))))
  (set `local.RandomValue` (`KismetMathLibrary.RandomIntegerInRange` 1 (`local.Sum`)))
  (bind _keys (`BlueprintMapLibrary.Map_Keys` _seedspawnchancemap))
  (for _array_element_2 _keys
    (bind _output_get (set `local.Max` (+ (`BlueprintMapLibrary.Map_Find` _seedspawnchancemap _array_element_2) (`local.Min`))))
    (if (and (> _randomvalue (`local.Min`)) (<= _randomvalue _output_get))
      (return _array_element_2)
      (else
        (set `local.Min` (`local.Max`)))))
  ;[1 1 1] Fallback
  (return "/Game/Blueprints/Actors/Pickups/BP_CornSeeds.BP_CornSeeds_C"))

(fn `GetSeedPoint`
  (returns (Output :type "Vector Structure"))
  (bind _seedpoint (`self.SeedPoint`))
  (bind (_returnvalue_x _returnvalue_y _returnvalue_z) (`KismetMathLibrary.BreakVector` (`SceneComponent.K2_GetComponentLocation` _seedpoint)))
  (bind (_returnvalue_x_2 _returnvalue_y_2) (`KismetMathLibrary.BreakVector` (+ (`SceneComponent.K2_GetComponentLocation` _seedpoint) (* (`KismetMathLibrary.RandomUnitVector`) (`self.SeedSpawnRadius`)))))
  (return (`KismetMathLibrary.MakeVector` _returnvalue_x_2 _returnvalue_y_2 _returnvalue_z)))

(fn `SaveState`
  (returns (OutSaveData :type "Array of InstancedStruct Structure"))
  (return))

(fn `UserConstructionScript`)