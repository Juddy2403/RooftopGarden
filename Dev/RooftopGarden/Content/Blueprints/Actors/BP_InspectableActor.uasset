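; Interactable prop that the player picks up to inspect and rotate in front of the view.
; Interact toggles viewing: it locks movement and vision, moves the actor along the look direction, then restores its saved transform on exit.
; While viewing, look input rotates it with left mouse or right shoulder held, and interaction feedback and HUD message are hidden.
; The construction script applies mesh, material and transform, and fits the box to mesh bounds.
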(event `self.ReceiveBeginPlay`
  (add `/Game/Blueprints/Components/BPC_InteractableFeedback.OnTick` (`self.BPC_InteractableFeedback`) (delegate `OnTick_Event`)))

(event `OnTick_Event`
  (bind _bpc_interactablefeedback (`self.BPC_InteractableFeedback`))
  (bind _returnvalue (`PlayerController.GetHUD` (`GameplayStatics.GetPlayerController` 0)))
  (if (`self.IsViewing`)
    (`/Game/Blueprints/Components/BPC_InteractableFeedback.SetInvisible` _bpc_interactablefeedback)
    (message `/Game/Blueprints/Interfaces/BPI_HudUtilities.SetHUDEnabled` _returnvalue false)
    (else
      (`/Game/Blueprints/Components/BPC_InteractableFeedback.SetVisible` _bpc_interactablefeedback)
      (message `/Game/Blueprints/Interfaces/BPI_HudUtilities.SetHUDEnabled` _returnvalue true))))

(event `GetOutOfViewMode`
  (bind _returnvalue (`GameplayStatics.GetPlayerCharacter` 0))
  (`CharacterMovementComponent.SetMovementMode` (`Character.CharacterMovement` _returnvalue) "MOVE_Walking" 0)
  (bind _asbp_first_person_character (cast `/Game/Blueprints/Pawns/BP_FirstPersonCharacter` _returnvalue))
  (`/Game/Blueprints/Pawns/BP_FirstPersonCharacter.LockVision` _asbp_first_person_character false)
  (clear `/Game/Blueprints/Pawns/BP_FirstPersonCharacter.OnLookInput` _asbp_first_person_character)
  (`self.K2_SetActorTransform` (`self.LastTransform`)))

(event `self.Interact`
  (params (InteractingActor :type "Actor Object Reference") (HeldItem :type "SlotStruct Structure"))
  (`/Engine/EditorBlueprintResources/StandardMacros.FlipFlop`
    (:`A`
      (set `self.IsViewing` true)
      (`self.GoInViewingMode`))
    (:`B`
      (set `self.IsViewing` false)
      (`self.GetOutOfViewMode`))))

(event `GoInViewingMode`
  (bind _returnvalue (`GameplayStatics.GetPlayerCharacter` 0))
  (`CharacterMovementComponent.DisableMovement` (`Character.CharacterMovement` _returnvalue))
  (bind _asbp_first_person_character (cast `/Game/Blueprints/Pawns/BP_FirstPersonCharacter` _returnvalue))
  (`/Game/Blueprints/Pawns/BP_FirstPersonCharacter.LockVision` _asbp_first_person_character true)
  (add `/Game/Blueprints/Pawns/BP_FirstPersonCharacter.OnLookInput` _asbp_first_person_character (delegate `OnLookInput_Event`))
  (set `self.LastTransform` (`self.GetTransform`))
  (bind (_startlocation _direction) (`UtilitiesLibrary.GetPlayerLookAt` (`GameplayStatics.GetPlayerController` 0)))
  (`self.K2_SetActorLocation` (+ _startlocation (* _direction (`self.DistanceFromPlayer`)))))

(event `OnLookInput_Event`
  (params (Value :type "Vector2D Structure"))
  (bind _returnvalue (`GameplayStatics.GetPlayerController` 0))
  (bind _rotationsensitivity (`self.RotationSensitivity`))
  (if (or (`PlayerController.IsInputKeyDown` _returnvalue "LeftMouseButton") (`PlayerController.IsInputKeyDown` _returnvalue "Gamepad_RightShoulder"))
    (`self.K2_AddActorWorldRotation` (`KismetMathLibrary.MakeRotator` 0.0 (* Value_Y _rotationsensitivity -1.0) (* Value_X _rotationsensitivity)))))

(fn `UserConstructionScript`
  (bind _staticmesh (`self.StaticMesh`))
  (bind _box (`self.Box`))
  (bind _meshworldtransform (`self.MeshWorldTransform`))
  (bind (_origin _boxextent) (`KismetSystemLibrary.GetComponentBounds` _staticmesh))
  (bind (_returnvalue_x _returnvalue_y _returnvalue_z) (`KismetMathLibrary.BreakVector` (* _boxextent 1.0)))
  (`StaticMeshComponent.SetStaticMesh` _staticmesh (`self.Mesh`))
  (`SceneComponent.K2_SetWorldLocation` _box _origin false false)
  (`BoxComponent.SetBoxExtent` _box (`KismetMathLibrary.MakeVector` _returnvalue_x 10.0 _returnvalue_z) true)
  (`PrimitiveComponent.SetMaterial` (`self.StaticMesh`) 0 (`self.MeshMaterial`))
  (if (not (== _meshworldtransform (`KismetMathLibrary.MakeTransform` (0.0 0.0 0.0))))
    (`SceneComponent.K2_SetWorldTransform` (`self.StaticMesh`) _meshworldtransform false false)))