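; Character component that runs ladder climbing for the first-person player, adding the ladder input context and blending onto the ladder spline on BeginPlay.
; Climb input applies vertical impulses, flipped when the camera looks down, while Tick snaps the character to the nearest spline point and a looping-state sound follows input.
; Reaching either end while moving outward blends the player off and destroys the component.
; The jump-off dismount logic is left unconnected.
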(event `self.ReceiveTick`
  (params (DeltaSeconds :type "Float (single-precision)"))
  (bind _lastinput (`self.LastInput`))
  (bind _ladder (`self.Ladder`))
  (bind _returnvalue (`Actor.K2_GetActorLocation` (`self.Owner Character`)))
  (bind _spline (`/Game/Blueprints/Actors/BP_Ladder.Spline` (`self.Ladder`)))
  (bind _returnvalue_2 (and (== _returnvalue (`SplineComponent.GetLocationAtSplinePoint` _spline 0 "World") :`ErrorTolerance` 4.0) (== _lastinput -1.0)))
  (`Actor.K2_SetActorLocation` (`self.Owner Character`) (`SplineComponent.FindLocationClosestToWorldLocation` (`/Game/Blueprints/Actors/BP_Ladder.Spline` (`self.Ladder`)) _returnvalue "World") false false)
  (if (or (and (== _returnvalue (`SplineComponent.GetLocationAtSplinePoint` _spline 1 "World") :`ErrorTolerance` 4.0) (== _lastinput 1.0)) _returnvalue_2)
    (`EnhancedInputSubsystemInterface.RemoveMappingContext` (pcsubsystem `EnhancedInputLocalPlayerSubsystem` (`self.Owner Controller`)) "/Game/Input/IMC_Ladder.IMC_Ladder" (struct))
    (`/Game/Blueprints/Pawns/BP_FirstPersonCharacter.ClimbBlend` (`self.Owner Character`) false (`Actor.K2_GetActorLocation` (`self.Owner Character`)) (select `bool` _returnvalue_2 :`false` (`SceneComponent.K2_GetComponentLocation` (`/Game/Blueprints/Actors/BP_Ladder.EndPoint` _ladder)) :`true` (`SceneComponent.K2_GetComponentLocation` (`/Game/Blueprints/Actors/BP_Ladder.Beginpoint` _ladder))) 0.25)
    (bind _climbingsound (`self.ClimbingSound`)
      (:`then`
        (`AudioComponent.Stop` _climbingsound))
      (:`else`
        _))
    (`self.K2_DestroyComponent`)))

(event `self.ReceiveBeginPlay`
  (bind _owner_character (`self.Owner Character`))
  (bind _returnvalue (`Actor.K2_GetActorLocation` _owner_character))
  (bind _asbp_first_person_character (cast `/Game/Blueprints/Pawns/BP_FirstPersonCharacter` (`self.GetOwner`) :!pure true))
  (bind _returnvalue_2 (`GameplayStatics.SpawnSound2D` "/Game/Audio/SoundCues/SC_Climbing.SC_Climbing" 1.0 1.0 0.0 null))
  (set `self.ClimbingSound` _returnvalue_2)
  (set `self.Owner Character` _asbp_first_person_character)
  (bind _output_get (set `self.Owner Controller` (cast `/Game/Blueprints/Game/BP_FirstPersonPlayerController` (`Pawn.GetController` _asbp_first_person_character) :!pure true)))
  (`EnhancedInputSubsystemInterface.AddMappingContext` (pcsubsystem `EnhancedInputLocalPlayerSubsystem` _output_get) "/Game/Input/IMC_Ladder.IMC_Ladder" 1 (struct))
  (`/Game/Blueprints/Pawns/BP_FirstPersonCharacter.ClimbBlend` _owner_character true _returnvalue (`SplineComponent.FindLocationClosestToWorldLocation` (`/Game/Blueprints/Actors/BP_Ladder.Spline` (`self.Ladder`)) _returnvalue "World") 0.25))

(event `EnhancedInput|/Game/Input/Actions/IA_Climb`
  (params (ActionValue :type "Float (double-precision)") (ElapsedSeconds :type "Float (double-precision)") (TriggeredSeconds :type "Float (double-precision)") (InputAction :type "InputAction Object Reference" :default "/Game/Input/Actions/IA_Climb.IA_Climb"))
  ;[1 1 1] Climbing
  (:`Triggered`
    (bind _output_get (set `self.LastInput` (select `bool` (`self.IsPlayerLookingUp`) :`false` (* ActionValue -1.0) :`true` ActionValue)))
    (`CharacterMovementComponent.AddImpulse` (`Character.CharacterMovement` (`self.Owner Character`)) (`KismetMathLibrary.MakeVector` 0.0 0.0 (* _output_get ElapsedSeconds (`self.ClimbSpeed`))) true))
  (:`Started`
    (bind _climbingsound (`self.ClimbingSound`)
      (:`then`
        (`AudioComponent.Play` _climbingsound 0.0))
      (:`else`)))
  (:`Canceled`
    (`self.ClimbingSound` :!label _label
      (:`then`
        (`AudioComponent.Stop` _climbingsound))
      (:`else`
        _))
    (`MovementComponent.StopMovementImmediately` (`Character.CharacterMovement` (`self.Owner Character`))))
  (:`Completed`
    (goto _label)))

(event `EnhancedInput|/Game/Input/Actions/IA_Dismount_Ladder`
  (params (ActionValue :type Boolean) (ElapsedSeconds :type "Float (double-precision)") (TriggeredSeconds :type "Float (double-precision)") (InputAction :type "InputAction Object Reference" :default "/Game/Input/Actions/IA_Dismount_Ladder.IA_Dismount_Ladder"))
  ;[1 1 1] Jump off ladder
)

(fn `Dismount Ladder`
  (`EnhancedInputSubsystemInterface.RemoveMappingContext` (pcsubsystem `EnhancedInputLocalPlayerSubsystem` (`self.Owner Controller`)) "/Game/Input/IMC_Ladder.IMC_Ladder" (struct))
  (`CharacterMovementComponent.SetMovementMode` (`Character.CharacterMovement` (`self.Owner Character`)) "MOVE_Walking" 0)
  (`self.K2_DestroyComponent`))

(fn `IsPlayerLookingUp`
  (returns (Result :type Boolean))
  (return (> (`KismetMathLibrary.Dot_VectorVector` (`KismetMathLibrary.GetForwardVector` (`PlayerCameraManager.GetCameraRotation` (`GameplayStatics.GetPlayerCameraManager` 0))) (`KismetMathLibrary.Vector_Up`)) 0.0)))