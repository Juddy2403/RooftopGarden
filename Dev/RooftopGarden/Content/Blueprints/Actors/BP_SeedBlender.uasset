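; Interactable seed blender that turns the player's produce into seeds, and seeds, bugs or weeds into fertilizer, pesticide or herbicide.
; Interact matches held Food to DT_PlantInfo for a random seed count, then checks inventory quantities for each product recipe.
; Blending plays audio, waits a delay derived from the sound's length, then spawns results scattered around SeedSpawnPoint.
; A feedback component shows the blend prompt while a non-tool item is active.
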(event `StartBlending`
  (params (Amount :type Integer) (ResultClass :type "Actor Class Reference"))
  (`AudioComponent.Play` (`self.Audio`) 0.0)
  (`KismetSystemLibrary.Delay` (`self.TimeToBlend`))
  (`self.SpawnItems` ResultClass Amount))

(event `SpawnItems`
  (params (Class :type "Actor Class Reference") (Amount :type Integer))
  (bind _seedspawnpoint (`self.SeedSpawnPoint`))
  (bind (_returnvalue_x _returnvalue_y _returnvalue_z) (`KismetMathLibrary.BreakVector` (`SceneComponent.K2_GetComponentLocation` _seedspawnpoint)))
  (bind (_returnvalue_x_2 _returnvalue_y_2) (`KismetMathLibrary.BreakVector` (+ (`SceneComponent.K2_GetComponentLocation` _seedspawnpoint) (* (`KismetMathLibrary.RandomUnitVector`) (`self.SeedSpawnRadius`)))))
  (for _ (range 1 (+ Amount 1))
    (`|SpawnActorFromClass` Class (`KismetMathLibrary.MakeTransform` (`KismetMathLibrary.MakeVector` _returnvalue_x_2 _returnvalue_y_2 _returnvalue_z)) "AdjustIfPossibleButAlwaysSpawn" "MultiplyWithRoot" null null)))

(event `OnFeedbackUpdate`
  (bind _bpc_interactablefeedback (`self.BPC_InteractableFeedback`))
  (bind (_itemstruct _returnvalue) (`UtilitiesLibrary.GetActiveItemInfoStruct` (`self.PlayerInventory`)))
  (if (and (`|EnumInequality` (`.ItemType` (break `ItemStruct` _itemstruct)) "Tool") _returnvalue)
    (`/Game/Blueprints/Components/BPC_InteractableFeedback.UpdateText` _bpc_interactablefeedback "Press" "/Game/Input/Actions/IA_Interact.IA_Interact" "blend")
    (`/Game/Blueprints/Components/BPC_InteractableFeedback.SetVisible` _bpc_interactablefeedback)
    (else
      (`/Game/Blueprints/Components/BPC_InteractableFeedback.SetInvisible` _bpc_interactablefeedback))))

(event `self.ReceiveBeginPlay`
  (bind _bpc_interactablefeedback (`self.BPC_InteractableFeedback`))
  (bind _returnvalue (`self.GetComponentByClass` (`GameplayStatics.GetPlayerPawn` 0) "/Script/RooftopGarden.InventoryComponent"))
  (add `/Game/Blueprints/Components/BPC_InteractableFeedback.OnEnabled` _bpc_interactablefeedback (delegate `OnFeedbackUpdate`))
  (add `/Game/Blueprints/Components/BPC_InteractableFeedback.OnTick` _bpc_interactablefeedback (delegate `OnFeedbackUpdate`))
  (`/Engine/EditorBlueprintResources/StandardMacros.IsValid` _returnvalue
    (:`Is Valid`
      (set `self.PlayerInventory` _returnvalue))))

(event `self.Interact`
  (params (InteractingActor :type "Actor Object Reference") (HeldItem :type "SlotStruct Structure"))
  (bind _returnvalue (`self.GetComponentByClass` InteractingActor "/Script/RooftopGarden.InventoryComponent"))
  (bind (_slotstruct_itemid _slotstruct_quantity) (break `SlotStruct` (`InventoryComponent.GetActiveSlotInfo` _returnvalue)))
  (`/Engine/EditorBlueprintResources/StandardMacros.IsValid` _returnvalue
    (:`Is Valid`
      (if (> _slotstruct_quantity 0)
        (bind _itemstruct (`UtilitiesLibrary.GetActiveItemInfoStruct` _returnvalue))
        (`|ExecutionSequence`
          (:`then_0`
            (if (`|EnumEquality` (`.ItemType` (break `ItemStruct` _itemstruct)) "Food")
              (bind _outrownames (`DataTableFunctionLibrary.GetDataTableRowNames` "/Game/Blueprints/DataTypes/DT_PlantInfo.DT_PlantInfo"))
              (for _array_element _outrownames
                (bind _returnvalue_2 (`|GetDataTableRow` "/Game/Blueprints/DataTypes/DT_PlantInfo.DT_PlantInfo" _array_element)
                  (:`then`
                    (if (== (break `ItemStruct` _itemstruct) (`.ProduceID` (break `PlantInfoStruct` _returnvalue_2)))
                      (bind _itemstruct_2 (`UtilitiesLibrary.GetActiveItemInfoStructFromID` _array_element))
                      (`InventoryComponent.RemoveFromActiveSlot` _returnvalue 1 true)
                      (break)))))
              (`self.StartBlending` (`KismetMathLibrary.RandomIntegerInRange` (`self.MinSeedsSpawned`) (`self.MaxSeedsSpawned`)) (`.ItemClass` (break `ItemStruct` _itemstruct_2)))))
          (:`then_1`
            (`self.TryToProcess` "Seed" (`self.NeededSeeds`) "/Game/Blueprints/Actors/Pickups/BP_Fertilizer.BP_Fertilizer_C" _returnvalue)
            (`self.TryToProcess` "Bug" (`self.NeededBugs`) "/Game/Blueprints/Actors/Pickups/BP_Pesticide.BP_Pesticide_C" _returnvalue)
            (`self.TryToProcess` "Weed" (`self.NeededWeeds`) "/Game/Blueprints/Actors/Pickups/BP_Herbicide.BP_Herbicide_C" _returnvalue)))))))

(event `TryToProcess`
  (params (ItemType :type "EItemType Enum" :default "Seed") (NeededQuantity :type Integer) (Result :type "Actor Class Reference") (Inventory :type "InventoryComponent Object Reference"))
  (if (`InventoryComponent.HasItemsOfType` Inventory ItemType NeededQuantity)
    (`InventoryComponent.RemoveItemsOfType` Inventory ItemType NeededQuantity)
    (`self.StartBlending` 1 Result)))

(fn `UserConstructionScript`
  (set `self.TimeToBlend` (* (`SoundBase.Duration` (`AudioComponent.Sound` (`self.Audio`))) 0.7)))