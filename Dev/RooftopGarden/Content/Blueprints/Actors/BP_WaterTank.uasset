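; BP_WaterTank is a water tank actor that shows interaction feedback only while the player holds a watering can.
; On BeginPlay it binds a check to the tick of its BPCInteractableFeedback component, toggling that feedback's visibility.
; The check calls HasWateringCan, which looks up the pawn's InventoryComponent, tests the active slot for the watering can item and also returns that actor.
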(event `FeedbackTextCheck`
  (bind _bpc_interactablefeedback (`self.BPC_InteractableFeedback`))
  (if (`self.HasWateringCan` (`GameplayStatics.GetPlayerPawn` 0))
    (`/Game/Blueprints/Components/BPC_InteractableFeedback.SetVisible` _bpc_interactablefeedback)
    (else
      (`/Game/Blueprints/Components/BPC_InteractableFeedback.SetInvisible` _bpc_interactablefeedback))))

(event `self.ReceiveBeginPlay`
  (add `/Game/Blueprints/Components/BPC_InteractableFeedback.OnTick` (`self.BPC_InteractableFeedback`) (delegate `FeedbackTextCheck`)))

(fn `HasWateringCan`
  (params (Actor :type "Actor Object Reference"))
  (returns (Result :type Boolean) (WateringCan :type "Actor Object Reference"))
  (bind _returnvalue (`self.GetComponentByClass` Actor "/Script/RooftopGarden.InventoryComponent"))
  (bind (_bisvalid _outactor) (`InventoryComponent.GetActiveSlotActor` _returnvalue))
  (bind _slotstruct_itemid (break `SlotStruct` (`InventoryComponent.GetActiveSlotInfo` _returnvalue)))
  (`/Engine/EditorBlueprintResources/StandardMacros.IsValid` _returnvalue
    (:`Is Valid`
      (return (and _bisvalid (== _slotstruct_itemid "watering_can")) _outactor))))

(fn `UserConstructionScript`)